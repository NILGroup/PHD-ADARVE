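; Experiment setup manager that picks the participant for a research session and launches the scenario.
; On BeginPlay it loads groups, per-group user IDs and last-session data from JSON, then initializes the setup panel widget.
; User selection alternates between groups or stays within one, tracking clamped per-group indices and updating the GameInstance.
; Starting saves session JSON, writes recording-system ID and group files, creates the user's database folder, then opens the next level.
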(event Custom|InitExperimentSetUpPanel
  (bind _aswbp_experiment_set_up_panel (Utilities|Casting|CastToWBP_ExperimentSetUpPanel (UserInterface|GetWidget (Variables|Default|GetWidget))))
  (bind _output_get (Variables|Default|SetExperimentSetUpWidget _aswbp_experiment_set_up_panel))
  (Variables|/Game/Experiment/UI/WBP_ExperimentSetUpPanel.WBP_ExperimentSetUpPanel_C|SetExperimentSetUpManager _output_get self)
  (Default|Init (Variables|Default|GetExperimentSetUpWidget)))

(event Custom|SetLastExperimentData
  (ReadDataFromFile|ReadLastExperimentInfofromFile)
  (Variables|ExperimentData|SetCurrentExperimentData (Variables|ExperimentData|GetLastExperimentData)))

(event Custom|LoadNextLevel
  (bind _output_get (Variables|/Game/Game/Blueprints/RR_GameInstance.RR_GameInstance_C|SetLevel%20to%20Load (CallFunction|GetMyGameInstance) (.BPLevelName (Utilities|Struct|BreakF_ScenarioData (.Next%20Scenario%20Data (CallFunction|GetCurrentScenarioNextData))))))
  (Game|OpenLevel(byName) _output_get))

(event Custom|StartExperiment
  (SaveDataToFile|WriteExperimentInfotoFile)
  (ChangeUser|ChangeRecordingSystemData)
  (CallFunction|CreateUserinDB)
  (Utilities|FlowControl|Delay 1.5)
  (CallFunction|LoadNextLevel))

(event Custom|CreateUserInDB
  (Class|RRFileManager|CreateDirectory (CallFunction|GetExperimentDirectory) "database")
  (Class|RRFileManager|CreateDirectory (CallFunction|GetExperimentDirectory) (Utilities|String|Append "database/" (Variables|/Game/Game/Blueprints/RR_GameInstance.RR_GameInstance_C|GetUserID (CallFunction|GetMyGameInstance)))))

(event Custom|SetCurrentUser
  (params (CurrentUserAndGroupData :type F%20User%20and%20Group%20Info%20Structure))
  (CurrentInfo|SetUserandGroupNewInfo CurrentUserAndGroupData))

(event EventBeginPlay
  (ReadDatafromFile|ReadExperimentGroupsfromFile)
  (ReadDatafromFile|ReadIdsbyGroupfromFile)
  (CallFunction|SetLastExperimentData)
  (CallFunction|InitExperimentSetUpPanel))

(fn ConstructionScript)

(fn GetUserIDListbyGroupType
  (params (GroupType :type E_UserGroup%20Enum :default "NewEnumerator0"))
  (bind _useridslists (Variables|UserIDs|GetUserIDsLists))
  (bind (_value _returnvalue) (Utilities|Map|Find _useridslists GroupType))
  (if _returnvalue
    (return (Utilities|Struct|BreakF_IDsList _value))
    (else
      (return 0))))

(fn GetUserIDbyIndex
  (params (GroupType :type E_UserGroup%20Enum :default "NewEnumerator0") (Index :type Integer))
  (return (Utilities|Array|Get(acopy) (CallFunction|GetUserIDListbyGroupType GroupType) Index)))

(fn GetNextUser
  (params (SelectionType :type E_UserSelectionType%20Enum :default "NewEnumerator0") (Increase :type Integer))
  (bind _data (CurrentInfo|GetCurrentUserandGroupInfo))
  (Utilities|FlowControl|Sequence
    (:then_0
      (switch Utilities|FlowControl|Switch|SwitchonE_UserSelectionType SelectionType
        (:NewEnumerator0
          (bind (_nextgroup _nextuserindexbygroup) (ChangeUser|GetNextAlternateUser (.grouptype _data) (.indexbygroup _data) Increase))
          (LocalVariables|SetNextUserGroup _nextgroup)
          (LocalVariables|SetIndexesUpdated _nextuserindexbygroup))
        (:NewEnumerator1
          (bind (_nextgroup_2 _nextuserindexbygroup_2) (ChangeUser|GetNextContinuousUser (.grouptype _data) (.indexbygroup _data) Increase))
          (LocalVariables|SetNextUserGroup _nextgroup_2)
          (LocalVariables|SetIndexesUpdated _nextuserindexbygroup_2))))
    (:then_1
      (CallFunction|SetCurrentUser (Utilities|Struct|MakeF_UserAndGroupInfo (ChangeUser|GetNextUserID (LocalVariables|GetNextUserGroup) (LocalVariables|GetIndexesUpdated)) (LocalVariables|GetNextUserGroup) "" SelectionType (LocalVariables|GetIndexesUpdated)))
      (return (Utilities|Struct|MakeF_UserAndGroupInfo (ChangeUser|GetNextUserID (LocalVariables|GetNextUserGroup) (LocalVariables|GetIndexesUpdated)) (LocalVariables|GetNextUserGroup) "" SelectionType (LocalVariables|GetIndexesUpdated))))))

(fn GetNextAlternateUser
  (params (CurrentGroup :type E_UserGroup%20Enum :default "NewEnumerator0") (UserIndexByGroup :type Map%20of%20E_UserGroup%20Enums%20to%20Integers :default "NewEnumerator0") (Increase :type Integer))
  (bind _result (Math|Integer|IncrementInt (Utilities|Array|FindItem (Variables|ExperimentData|GetExperimentGroupTypeList) CurrentGroup))
    (:%20%20
      (Utilities|Map|Add UserIndexByGroup (Utilities|Array|Get(acopy) (Variables|ExperimentData|GetExperimentGroupTypeList) (CallFunction|WrapInteger _result 0 (Utilities|Array|Length (Variables|ExperimentData|GetExperimentGroupTypeList)))) (Math|Integer|Clamp(Integer) (+ (.Value (Utilities|Map|Find UserIndexByGroup (Utilities|Array|Get(acopy) (Variables|ExperimentData|GetExperimentGroupTypeList) (CallFunction|WrapInteger _result 0 (Utilities|Array|Length (Variables|ExperimentData|GetExperimentGroupTypeList)))))) Increase) 0 (- (Utilities|Array|Length (CallFunction|GetUserIDListbyGroupType (Utilities|Array|Get(acopy) (Variables|ExperimentData|GetExperimentGroupTypeList) (CallFunction|WrapInteger _result 0 (Utilities|Array|Length (Variables|ExperimentData|GetExperimentGroupTypeList)))))) 1)))
      (return (Utilities|Array|Get(acopy) (Variables|ExperimentData|GetExperimentGroupTypeList) (CallFunction|WrapInteger _result 0 (Utilities|Array|Length (Variables|ExperimentData|GetExperimentGroupTypeList)))) UserIndexByGroup))))

(fn GetNextContinuousUser
  (params (CurrentGroup :type E_UserGroup%20Enum :default "NewEnumerator0") (UserIndexByGroup :type Map%20of%20E_UserGroup%20Enums%20to%20Integers :default "NewEnumerator0") (Increase :type Integer))
  (Utilities|Map|Add UserIndexByGroup CurrentGroup (Math|Integer|Clamp(Integer) (+ (.Value (Utilities|Map|Find UserIndexByGroup CurrentGroup)) Increase) 0 (- (Utilities|Array|Length (CallFunction|GetUserIDListbyGroupType CurrentGroup)) 1)))
  (return CurrentGroup UserIndexByGroup))

(fn GetNextUserID
  (params (NextUserGroup :type E_UserGroup%20Enum :default "NewEnumerator0") (NextUserIndexByGroup :type Map%20of%20E_UserGroup%20Enums%20to%20Integers :default "NewEnumerator0"))
  (return (Utilities|Array|Get(acopy) (CallFunction|GetUserIDListbyGroupType NextUserGroup) (.Value (Utilities|Map|Find NextUserIndexByGroup NextUserGroup)))))

(fn ResetCurrentUser
  (CallFunction|SetCurrentUser (.userandgroup (Variables|ExperimentData|GetLastExperimentData))))

(fn UserExistsinLocalFileDatabase
  (return (Class|RRFileManager|DirectoryExists (Utilities|String|Append (CallFunction|GetExperimentDirectory) "/database") (Variables|/Game/Game/Blueprints/RR_GameInstance.RR_GameInstance_C|GetUserID (CallFunction|GetMyGameInstance)))))

(fn ReadLastExperimentInfofromFile
  (bind _outjsonobject (Class|JsonBlueprintFunctionLibrary|FromFile (Utilities|Struct|MakeFilePath (Utilities|String|Append (CallFunction|GetExperimentDirectory) "/data/last_experiment.json"))))
  (bind _outvalue (|GetJsonField _outjsonobject "ResearcherAndExperiment"))
  (bind _outvalue_2 (|GetJsonField _outjsonobject "UserAndGroup"))
  (Variables|ExperimentData|SetLastExperimentData (Utilities|Struct|MakeF_ExperimentInfo (ReadDataFromFile|ReadLastResearcherandExperimentInfofromFile _outvalue) (ReadDataFromFile|ReadLastUserandGroupInfofromFile _outvalue_2))))

(fn ReadLastResearcherandExperimentInfofromFile
  (params (Json%20Object :type Json%20Object%20Wrapper%20Structure))
  (Utilities|FlowControl|Sequence
    (:then_0
      (bind _outvalue (|GetJsonField Json%20Object "ResearcherName"))
      (LocalVariables|SetResearcherName _outvalue))
    (:then_1
      (bind _outvalue_2 (|GetJsonField Json%20Object "ComputerID"))
      (LocalVariables|SetComputerID _outvalue_2))
    (:then_2
      (bind _outvalue_3 (|GetJsonField Json%20Object "ExperimentID"))
      (LocalVariables|SetExperimentID _outvalue_3))
    (:then_3
      (bind _outvalue_4 (|GetJsonField Json%20Object "SessionID"))
      (LocalVariables|SetSessionID _outvalue_4))
    (:then_4
      (return (Utilities|Struct|MakeF_ResearcherAndExperimentInfo (LocalVariables|GetResearcherName) (LocalVariables|GetComputerID) (LocalVariables|GetExperimentID) (LocalVariables|GetSessionID))))))

(fn ReadLastUserandGroupInfofromFile
  (params (Json%20Object :type Json%20Object%20Wrapper%20Structure))
  (Utilities|FlowControl|Sequence
    (:then_0
      (bind _outvalue (|GetJsonField Json%20Object "UserID"))
      (LocalVariables|SetUserID _outvalue))
    (:then_1
      (bind _outvalue_2 (|GetJsonField Json%20Object "GroupType"))
      (LocalVariables|SetGroupType (CallFunction|GetGroupTypefromString _outvalue_2)))
    (:then_2
      (bind _outvalue_3 (|GetJsonField Json%20Object "Date"))
      (LocalVariables|SetDate _outvalue_3))
    (:then_3
      (bind _outvalue_4 (|GetJsonField Json%20Object "UserSelectionType"))
      (LocalVariables|SetUserSelectionType (CallFunction|GetUserSelectionTypefromString _outvalue_4)))
    (:then_4
      (bind _outvalue_5 (|GetJsonField Json%20Object "IndexByGroup"))
      (bind _fieldnames (Class|JsonBlueprintFunctionLibrary|GetFieldNames _outvalue_5))
      (for _array_element _fieldnames
        (bind _outvalue_6 (|GetJsonField _outvalue_5 _array_element))
        (Utilities|Map|Add (LocalVariables|GetIndexByGroup) (CallFunction|GetGroupTypefromString _array_element) _outvalue_6)))
    (:then_5
      (return (Utilities|Struct|MakeF_UserAndGroupInfo (LocalVariables|GetUserID) (LocalVariables|GetGroupType) (LocalVariables|GetDate) (LocalVariables|GetUserSelectionType) (LocalVariables|GetIndexByGroup))))))

(fn GetGroupTypefromString
  (params (GroupType_S :type String))
  (bind _enumvalue (|ForEachE_UserGroup)
    (:LoopBody
      (if (Utilities|Enum|Equal(Enum) (Utilities|String|EnumtoString _enumvalue) GroupType_S)
        (return _enumvalue)))))

(fn GetUserSelectionTypefromString
  (params (UserSelectionType_S :type String))
  (bind _enumvalue (|ForEachE_UserSelectionType)
    (:LoopBody
      (if (Utilities|Enum|Equal(Enum) (Utilities|String|EnumtoString _enumvalue) UserSelectionType_S)
        (return _enumvalue)))))

(fn ReadIdsbyGroupfromFile
  (bind _outjsonobject (Class|JsonBlueprintFunctionLibrary|FromFile (Utilities|Struct|MakeFilePath (Utilities|String|Append (CallFunction|GetExperimentDirectory) "/data/users_ids_by_group.json"))))
  (bind _fieldnames (Class|JsonBlueprintFunctionLibrary|GetFieldNames _outjsonobject))
  (for _array_element _fieldnames
    (bind _outvalue (|GetJsonField _outjsonobject _array_element))
    (Utilities|Map|Add (Variables|UserIDs|GetUserIDsLists) (CallFunction|GetGroupTypefromString _array_element) (Utilities|Struct|MakeF_IDsList _outvalue))))

(fn ChangeRecordingSystemData
  (bind _data (CurrentInfo|GetCurrentUserandGroupInfo))
  (Class|RRFileManager|WriteFile (Utilities|String|Append (CallFunction|GetExperimentDirectory) (LocalVariables|GetUserIdFilePath)) (.userid _data))
  (Class|RRFileManager|WriteFile (Utilities|String|Append (CallFunction|GetExperimentDirectory) (LocalVariables|GetGroupTypeFilePath)) (Utilities|String|EnumtoString (.grouptype _data))))

(fn WriteExperimentInfotoFile
  (|SetJsonField (LocalVariables|GetData) "ResearcherAndExperiment" (SaveDatatoFile|WriteResearcherandExperimentInfotoFile))
  (|SetJsonField (LocalVariables|GetData) "UserAndGroup" (SaveDatatoFile|WriteUserandGroupInfotoFile))
  (Class|JsonBlueprintFunctionLibrary|ToFile (LocalVariables|GetData) (Utilities|Struct|MakeFilePath (Utilities|String|Append (CallFunction|GetExperimentDirectory) "/data/last_experiment.json"))))

(fn WriteUserandGroupInfotoFile
  (bind _currentexperimentdata (Variables|ExperimentData|GetCurrentExperimentData))
  (bind _currentexperimentdata_2 (Variables|ExperimentData|GetCurrentExperimentData))
  (Utilities|FlowControl|Sequence
    (:then_0
      (|SetJsonField (LocalVariables|GetJsonObject) "UserID" (.userid (.userandgroup _currentexperimentdata_2)))
      (|SetJsonField (LocalVariables|GetJsonObject) "GroupType" (Utilities|String|EnumtoString (.grouptype (.userandgroup _currentexperimentdata_2))))
      (|SetJsonField (LocalVariables|GetJsonObject) "Date" (CallFunction|ConvertDatetimetoString (Math|DateTime|Now) false))
      (|SetJsonField (LocalVariables|GetJsonObject) "UserSelectionType" (Utilities|String|EnumtoString (.userselectiontype (.userandgroup _currentexperimentdata_2)))))
    (:then_1
      (bind _enumvalue (|ForEachE_UserGroup)
        (:LoopBody
          (|SetJsonField (LocalVariables|GetIdsByGroup) (Utilities|String|EnumtoString _enumvalue) (.Value (Utilities|Map|Find (.indexbygroup (.userandgroup (Variables|ExperimentData|GetLastExperimentData))) _enumvalue))))
        (:then
          (|SetJsonField (LocalVariables|GetIdsByGroup) (Utilities|String|EnumtoString (.grouptype (.userandgroup _currentexperimentdata))) (.Value (Utilities|Map|Find (.indexbygroup (.userandgroup _currentexperimentdata)) (.grouptype (.userandgroup _currentexperimentdata)))))
          (|SetJsonField (LocalVariables|GetJsonObject) "IndexByGroup" (LocalVariables|GetIdsByGroup)))))
    (:then_2
      (return (LocalVariables|GetJsonObject)))))

(fn WriteResearcherandExperimentInfotoFile
  (bind _currentexperimentdata (Variables|ExperimentData|GetCurrentExperimentData))
  (|SetJsonField (LocalVariables|GetJsonObject) "ResearcherName" (.researchername (.researcherandexperiment _currentexperimentdata)))
  (|SetJsonField (LocalVariables|GetJsonObject) "ComputerID" (.computerid (.researcherandexperiment _currentexperimentdata)))
  (|SetJsonField (LocalVariables|GetJsonObject) "ExperimentID" (.experimentid (.researcherandexperiment _currentexperimentdata)))
  (|SetJsonField (LocalVariables|GetJsonObject) "SessionID" (.sessionid (.researcherandexperiment _currentexperimentdata)))
  (return (LocalVariables|GetJsonObject)))

(fn SetResearcherandExperimentNewInfo
  (params (NewData :type F%20Researcher%20and%20Experiment%20Info%20Structure))
  (Variables|ExperimentData|SetCurrentExperimentData (Utilities|Struct|MakeF_ExperimentInfo NewData (.userandgroup (Variables|ExperimentData|GetCurrentExperimentData)))))

(fn GetCurrentResearcherandExperimentInfo
  (return (.researcherandexperiment (Variables|ExperimentData|GetCurrentExperimentData))))

(fn SetUserandGroupNewInfo
  (params (Current%20Experiment%20Data%20User%20and%20Group :type F%20User%20and%20Group%20Info%20Structure))
  (bind _data (CurrentInfo|GetCurrentUserandGroupInfo))
  (bind _gameinstance (CallFunction|GetMyGameInstance))
  (bind (_userid _grouptype) (Utilities|Struct|BreakF_UserAndGroupInfo _data))
  (Variables|ExperimentData|SetCurrentExperimentData (Utilities|Struct|MakeF_ExperimentInfo (.researcherandexperiment (Variables|ExperimentData|GetCurrentExperimentData)) Current%20Experiment%20Data%20User%20and%20Group))
  (Variables|/Game/Game/Blueprints/RR_GameInstance.RR_GameInstance_C|SetUserID _gameinstance _userid)
  (Variables|/Game/Game/Blueprints/RR_GameInstance.RR_GameInstance_C|SetUserGroupType _gameinstance _grouptype)
  (Default|SetTutorialType _gameinstance)
  (Default|CallEDUserChanged _data))

(fn GetCurrentUserandGroupInfo
  (return (.userandgroup (Variables|ExperimentData|GetCurrentExperimentData))))

(fn ReadExperimentGroupsfromFile
  (bind _outjsonobject (Class|JsonBlueprintFunctionLibrary|FromFile (Utilities|Struct|MakeFilePath (Utilities|String|Append (CallFunction|GetExperimentDirectory) "/data/current_experiment_groups.json"))))
  (bind _outvalue (|GetJsonField _outjsonobject "Groups"))
  (bind _output_get (Variables|ExperimentData|SetExperimentGroupTypeList _outvalue))
  (for _array_element _output_get
    _))