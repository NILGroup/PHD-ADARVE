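; Manages a set of place points where VR players put pickable items of one type, tracking occupancy for an info widget.
; Binds to matching items' grab events to activate free points, deactivating them on release unless either hand still holds another such item.
; Point placed and removed events update the count and fire per-item and all-filled dispatchers.
; Placements and attempts are logged to the experiment database through the game instance.
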(event Custom|HideInfoWidget
  ;[1 1 1] Info Widget
  (Development|SetHiddeninGame (Variables|Default|GetPlacePointInfoWidgetComponent) true false))

(event Custom|BindActorEvents
  (params (Actor :type Actor%20Object%20Reference))
  (bind _yes (CallFunction|SameClass? (Utilities|GetClass Actor)))
  (if _yes
    (bind _asbp_pickable_item (Utilities|Casting|CastToBP_PickableItem Actor))
    (EventDispatchers|BindEventtoEDInteractionStarted _asbp_pickable_item (delegate Custom|OnActorGrabbed))
    (EventDispatchers|BindEventtoEDInteractionCompleted _asbp_pickable_item (delegate Custom|OnActorReleased))))

(event Custom|SetInfoWidgetData
  ;[1 1 1] Info Widget
  (bind _aswbp_place_point_info (Utilities|Casting|CastToWBP_PlacePointInfo (UserInterface|GetWidget (Variables|Default|GetPlacePointInfoWidgetComponent))))
  (bind _output_get (Variables|Default|SetPlacePointInfoWidget _aswbp_place_point_info))
  (Default|SetData _output_get (Utilities|Array|Length (Variables|Default|GetPlaceInPoints)) (Variables|Default|GetItemsName)))

(event Custom|UpdateInfoWidgetData
  ;[1 1 1] Info Widget
  (Default|UpdateNumOfItems (Variables|Default|GetPlacePointInfoWidget) (Variables|Default|GetCurrentNumOfPointsBeingUsed)))

(event Custom|OnItemSpawned
  (params (Actor :type BP%20Pickable%20Item%20Object%20Reference))
  (if (Utilities|Enum|Equal(Enum) (Variables|/Game/Game/Blueprints/Actors/Items/BP_InteractItemParent.BP_InteractItemParent_C|GetItemType Actor) (Variables|Default|GetItemType))
    (CallFunction|BindActorEvents Actor)))

(event Custom|OnActorGrabbed
  (params (Actor :type BP%20Interact%20Item%20Parent%20Object%20Reference))
  (if (Variables|Default|GetCanActivatePoints)
    (for _array_element (Variables|Default|GetPlaceInPoints)
      (if (not (Variables|/Game/Game/Blueprints/Actors/Items/PlacePoints/BP_PlacePoint.BP_PlacePoint_C|GetActorPlaced _array_element))
        (Default|ActivatePoint _array_element true)))))

(event Custom|OnItemTriedToPlace
  (params (Item :type BP%20Pickable%20Item%20Object%20Reference) (PlacePoint :type BP%20Place%20Point%20Object%20Reference))
  (CallFunction|SendPlacePointEventtoDataBase Item PlacePoint))

(event Custom|ShowInfoWidget
  ;[1 1 1] Info Widget
  (if (Variables|Default|GetInfoAvailable)
    (Development|SetHiddeninGame (Variables|Default|GetPlacePointInfoWidgetComponent) false false)))

(event Custom|OnActorReleased
  (params (Actor :type BP%20Interact%20Item%20Parent%20Object%20Reference))
  (bind _can_disable (CallFunction|CanDisablePlacePoints? Actor))
  (if _can_disable
    (for _array_element (Variables|Default|GetPlaceInPoints)
      (Default|ActivatePoint _array_element false))))

(event Custom|BindPlacePointsEvents
  (for _array_element (Variables|Default|GetPlaceInPoints)
    (EventDispatchers|BindEventtoEDItemPlaced _array_element (delegate Custom|OnItemPlaced))
    (EventDispatchers|BindEventtoEDItemRemoved _array_element (delegate Custom|OnItemRemoved))
    (EventDispatchers|BindEventtoEDItemTriedtoPlace _array_element (delegate Custom|OnItemTriedToPlace))))

(event Custom|OnItemPlaced
  (params (Item :type BP%20Pickable%20Item%20Object%20Reference) (PlacePoint :type BP%20Place%20Point%20Object%20Reference))
  (Default|CallEDOneItemHasBeenPlaced Item PlacePoint)
  (bind _result (Math|Integer|IncrementInt (Variables|Default|GetCurrentNumOfPointsBeingUsed))
    (:%20%20
      (Variables|Default|SetCurrentNumOfPointsBeingUsed _result)
      (CallFunction|UpdateInfoWidgetData)
      (Default|ActivatePoint PlacePoint false)
      (CallFunction|SendPlacePointEventtoDataBase Item PlacePoint)
      (bind _yes (CallFunction|AreAllPointsBeingUsed?))
      (bind _output_get (Variables|Default|SetAllPointsUsed _yes))
      (if _output_get
        (Default|CallEDAllPlacePointswithItems)))))

(event Custom|OnItemRemoved
  (params (Item :type BP%20Pickable%20Item%20Object%20Reference) (PlacePoint :type BP%20Place%20Point%20Object%20Reference))
  (Default|CallEDOneItemHasBeenRemoved Item PlacePoint)
  (Math|Integer|DecrementInt (Variables|Default|GetCurrentNumOfPointsBeingUsed)
    (:%20%20
      (Variables|Default|SetCurrentNumOfPointsBeingUsed 0)
      (CallFunction|UpdateInfoWidgetData)
      (Variables|Default|SetAllPointsUsed false)
      (Default|CallEDSomePlacePointsWithoutItems))))

(event Custom|InitPlacePoints
  (CallFunction|BindPlacePointsEvents)
  (for _array_element (Variables|Default|GetPlaceInPoints)
    (Variables|/Game/Game/Blueprints/Actors/Items/PlacePoints/BP_PlacePoint.BP_PlacePoint_C|SetPlaceItemManager _array_element self)
    (Default|ActivatePoint _array_element false)))

(event EventBeginPlay
  (Utilities|FlowControl|Sequence
    (:then_0
      (bind _asrr_game_instance (Utilities|Casting|CastToRR_GameInstance (Game|GetGameInstance)))
      (Variables|Default|SetGameInstance _asrr_game_instance))
    (:then_1
      (CallFunction|InitPlacePoints)
      (CallFunction|SetInfoWidgetData)
      (CallFunction|HideInfoWidget)
      (bind _outactors (Actor|GetAllActorsOfClass "/Game/Game/Blueprints/Actors/Items/BP_PickableItem.BP_PickableItem_C"))
      (for _array_element _outactors
        (bind _asbp_pickable_item (Utilities|Casting|CastToBP_PickableItem _array_element))
        (if (Utilities|Enum|Equal(Enum) (Variables|/Game/Game/Blueprints/Actors/Items/BP_InteractItemParent.BP_InteractItemParent_C|GetItemType _asbp_pickable_item) (Variables|Default|GetItemType))
          (CallFunction|BindActorEvents _array_element))))))

(fn ConstructionScript)

(fn SameClass?
  (params (Actor :type Actor%20Class%20Reference))
  (return (== Actor (Variables|Default|GetItemClass))))

(fn AreAllPointsBeingUsed?
  (for _array_element (Variables|Default|GetPlaceInPoints)
    (if (not (Variables|/Game/Game/Blueprints/Actors/Items/PlacePoints/BP_PlacePoint.BP_PlacePoint_C|GetActorPlaced _array_element))
      (return false)))
  (return true))

(fn ItemIsRelatedwithPoint?
  (params (Actor :type Actor%20Object%20Reference))
  (for _array_element (Variables|Default|GetPlaceInPoints)
    (if (== (Variables|/Game/Game/Blueprints/Actors/Items/PlacePoints/BP_PlacePoint.BP_PlacePoint_C|GetTargetPlaceActor _array_element) Actor)
      (return true)))
  (return false))

(fn SendPlacePointEventtoDataBase
  (params (Actor :type BP%20Pickable%20Item%20Object%20Reference) (PlacePoint :type BP%20Place%20Point%20Object%20Reference))
  (bind _data (Default|GetDataBaseMainInfoEvent (Variables|Default|GetGameInstance)))
  (bind _database_manager (Variables|/Game/Game/Blueprints/RR_GameInstance.RR_GameInstance_C|GetDatabase%20Manager (Variables|Default|GetGameInstance))
    (:then
      (Default|SendPlacePointEventtoDB _database_manager (Utilities|Struct|MakeF_PlacePointEvent 0 (.user_id (Utilities|Struct|BreakF_MainInfoEvent _data)) (.experiment_id (Utilities|Struct|BreakF_MainInfoEvent _data)) (.scenario_type (Utilities|Struct|BreakF_MainInfoEvent _data)) (Variables|/Game/Game/Blueprints/Actors/Items/BP_InteractItemParent.BP_InteractItemParent_C|GetActorId Actor) (Utilities|GetDisplayName Actor) (Utilities|GetDisplayName PlacePoint) (Variables|/Game/Game/Blueprints/Actors/Items/PlacePoints/BP_PlacePoint.BP_PlacePoint_C|GetNumOfActivation PlacePoint) (Variables|/Game/Game/Blueprints/Actors/Items/PlacePoints/BP_PlacePoint.BP_PlacePoint_C|GetStartActivationDatetime PlacePoint) (Math|DateTime|Now))))
    (:else)))

(fn CanDisablePlacePoints?
  (params (Actor :type BP%20Interact%20Item%20Parent%20Object%20Reference))
  (bind _asbp_player_vr (Utilities|Casting|CastToBP_Player_VR (Variables|/Game/Game/Blueprints/RR_GameInstance.RR_GameInstance_C|GetCurrentPlayer (Variables|Default|GetGameInstance))))
  (Utilities|FlowControl|Sequence
    (:then_0
      (LocalVariables|SetLeftItem (Variables|/Game/Game/Blueprints/Player/BP_Player_VR.BP_Player_VR_C|GetGrabbedItemL _asbp_player_vr))
      (LocalVariables|SetRightItem (Variables|/Game/Game/Blueprints/Player/BP_Player_VR.BP_Player_VR_C|GetGrabbedItemR _asbp_player_vr)))
    (:then_1
      (Utilities|IsValid (LocalVariables|GetLeftItem)
        (:Is%20Valid
          (if (!= (LocalVariables|GetLeftItem) Actor)
            (if (Utilities|Enum|Equal(Enum) (Variables|/Game/Game/Blueprints/Actors/Items/BP_InteractItemParent.BP_InteractItemParent_C|GetItemType (LocalVariables|GetLeftItem)) (Variables|Default|GetItemType))
              (return false))))))
    (:then_2
      (Utilities|IsValid (LocalVariables|GetRightItem)
        (:Is%20Valid
          (if (!= (LocalVariables|GetRightItem) Actor)
            (if (Utilities|Enum|Equal(Enum) (Variables|/Game/Game/Blueprints/Actors/Items/BP_InteractItemParent.BP_InteractItemParent_C|GetItemType (LocalVariables|GetRightItem)) (Variables|Default|GetItemType))
              (return false))))))
    (:then_3
      (return true))))