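; BP_Door is a door actor that a motion controller can swing by hand or that opens automatically.
; SetDoorOpenAngle sets the mesh yaw from the controller-to-door look-at angle minus an offset, clamped within 90 degrees either side of the rotation cached at BeginPlay.
; AutomaticOpenAndLockDoor plays the Open component and runs a timeline that lerps the door a quarter turn from that cached rotation; no lock logic appears here.
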(event Custom|AutomaticOpenAndLockDoor
  (bind _orirotation (Variables|Default|GetOriRotation))
  (bind (_roll _pitch _yaw) (Math|Rotator|BreakRotator _orirotation))
  (Audio|Components|Audio|Play (Variables|Default|GetOpen) 0.0)
  (bind _newtrack_0 (Timeline|OpenDoorTimeline PlayFromStart)
    (:Update
      (Transformation|SetWorldRotation (Variables|Default|GetDoorMesh) (Math|Rotator|Lerp(Rotator) _orirotation (Math|Rotator|MakeRotator _roll _pitch (+ _yaw -9e+01)) _newtrack_0) false false))))

(event EventBeginPlay
  (Variables|Default|SetOriRotation (Transformation|GetWorldRotation (Variables|Default|GetDoorMesh))))

(fn ConstructionScript)

(fn SetDoorOpenAngle
  (params (MotionController :type Motion%20Controller%20Component%20Object%20Reference) (AngleOffset :type Float%20%28double-precision%29))
  (bind _returnvalue (Transformation|GetWorldLocation MotionController))
  (bind _orirotation (Variables|Default|GetOriRotation))
  (bind _doormesh (Variables|Default|GetDoorMesh))
  (bind _returnvalue_2 (Transformation|GetWorldLocation _doormesh))
  (bind _returnvalue_3 (Math|Rotator|FindLookatRotation _returnvalue _returnvalue_2))
  (LocalVariables|SetCurrentAngleDifference (.yaw _returnvalue_3))
  (Transformation|SetWorldRotation (Variables|Default|GetDoorMesh) (Math|Rotator|MakeRotator 0.0 0.0 (Math|Float|ClampAngle (- (.yaw _returnvalue_3) AngleOffset) (- (.yaw _orirotation) 9e+01) (+ (.yaw _orirotation) 9e+01))) false false))