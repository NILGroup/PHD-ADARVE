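; Talkable NPC that offers a start-talking button when the player enters its TalkArea and runs conversations through a dialog widget.
; Button presses start the ACDialogManagerNPC component; leaving the area stops the dialog and hides the button.
; Dialog stopped and completed events both fire a conversation-finished dispatcher.
; Conversation starts and finishes are logged to the database with user, experiment, scenario and conversation index.
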(event OnComponentEndOverlap(TalkArea)
  (params (OverlappedComponent :type Primitive%20Component%20Object%20Reference) (OtherActor :type Actor%20Object%20Reference) (OtherComp :type Primitive%20Component%20Object%20Reference) (OtherBodyIndex :type Integer))
  ;[1 1 1] Talk Area
  (if (== OtherActor (CallFunction|GetMyPlayer))
    (Variables|Default|SetCanLookPlayer false)
    (Default|StopDialog (Variables|Default|GetAC_DialogManager_NPC))
    (Development|SetHiddeninGame (Variables|Default|GetStartTalkingButtonWidgetComponent) true false)))

(event OnComponentBeginOverlap(TalkArea)
  (params (OverlappedComponent :type Primitive%20Component%20Object%20Reference) (OtherActor :type Actor%20Object%20Reference) (OtherComp :type Primitive%20Component%20Object%20Reference) (OtherBodyIndex :type Integer) (bFromSweep :type Boolean) (SweepResult :type Hit%20Result%20Structure%20%28by%20ref%29))
  ;[1 1 1] Talk Area
  (if (== OtherActor (CallFunction|GetMyPlayer))
    (if (and (Variables|Default|GetCanTalk) (not (Variables|/Game/Game/Components/Dialogs/AC_DialogManager.AC_DialogManager_C|GetIsTalking? (Variables|Default|GetAC_DialogManager_NPC))))
      (Variables|Default|SetCanLookPlayer true)
      (Development|SetHiddeninGame (Variables|Default|GetStartTalkingButtonWidgetComponent) false false))))

(event Custom|NextConversation
  (Default|NextConversation (Variables|Default|GetAC_DialogManager_NPC)))

(event Custom|InitStartTalkingButton
  (Development|SetHiddeninGame (Variables|Default|GetStartTalkingButtonWidgetComponent) true false)
  (CallFunction|ShowHideDialogPanel false)
  (bind _aswbp_start_talking_button (Utilities|Casting|CastToWBP_StartTalkingButton (UserInterface|GetWidget (Variables|Default|GetStartTalkingButtonWidgetComponent))))
  (bind _output_get (Variables|Default|SetStartTalkingWidgetActor _aswbp_start_talking_button))
  (EventDispatchers|AssignEDStartTalking _output_get (delegate Custom|OnStartTalkingButtonPressed)))

(event Custom|OnDialogCompleted
  (params (DialogID :type Name))
  (CallFunction|ConversationFinished "None"))

(event Custom|OnStartTalkingButtonPressed
  (Development|SetHiddeninGame (Variables|Default|GetStartTalkingButtonWidgetComponent) true false)
  (Default|StartConversation (Variables|Default|GetAC_DialogManager_NPC))
  (CallFunction|SendDialogEventtoDB "NewEnumerator10" "Left"))

(event Custom|PlayerIsAlreadyOverlapping
  ;[1 1 1] Talk Area
  (if (Collision|IsOverlappingActor (Variables|Default|GetTalkArea) (CallFunction|GetMyPlayer) :!class /Script/Engine.PrimitiveComponent)
    (if (and (Variables|Default|GetCanTalk) (not (Variables|/Game/Game/Components/Dialogs/AC_DialogManager.AC_DialogManager_C|GetIsTalking? (Variables|Default|GetAC_DialogManager_NPC))))
      (Variables|Default|SetCanLookPlayer true)
      (Development|SetHiddeninGame (Variables|Default|GetStartTalkingButtonWidgetComponent) false false))))

(event Custom|SendDialogEventToDB
  (params (Event%20Type :type E_NPCEventType%20Enum :default "NewEnumerator5") (hand :type EControllerHand%20Enum :default "Left"))
  (bind _data (Default|GetDataBaseMainInfoEvent (CallFunction|GetMyGameInstance)))
  (Default|SendNPCInteractionEventtoDB (CallFunction|GetMyDatabase) (Utilities|Struct|MakeF_NPCInteractionEvent 0 (.user_id (Utilities|Struct|BreakF_MainInfoEvent _data)) (.experiment_id (Utilities|Struct|BreakF_MainInfoEvent _data)) (.scenario_type (Utilities|Struct|BreakF_MainInfoEvent _data)) (Variables|Default|GetActorId) (Variables|/Game/Game/Components/Dialogs/AC_DialogManager_NPC.AC_DialogManager_NPC_C|GetCurrentConversationIndex (Variables|Default|GetAC_DialogManager_NPC)) Event%20Type hand (Math|DateTime|Now))))

(event Custom|ShowHideDialogPanel
  (params (Show%20Dialog%20Panel :type Boolean))
  (bind _dialogwidgetcomponent (Variables|Default|GetDialogWidgetComponent))
  (if Show%20Dialog%20Panel
    (Development|SetHiddeninGame _dialogwidgetcomponent false false)
    (Default|ShowDialogBox (Variables|Default|GetDialogWidgetActor))
    (else
      (Development|SetHiddeninGame _dialogwidgetcomponent true false)
      (Default|HideDialogBox (Variables|Default|GetDialogWidgetActor)))))

(event Custom|Conversation%20Finished
  (params (Conversation%20ID :type Name))
  (Default|CallEDConversationFinished Conversation%20ID)
  (CallFunction|SendDialogEventtoDB "NewEnumerator28" "Left"))

(event Custom|OnDialogStopped
  (CallFunction|ConversationFinished "None"))

(event Custom|BindDialogEvents
  (bind _ac_dialogmanager_npc (Variables|Default|GetAC_DialogManager_NPC))
  (EventDispatchers|BindEventtoEDDialogStopped _ac_dialogmanager_npc (delegate Custom|OnDialogStopped))
  (EventDispatchers|BindEventtoEDDialogCompleted _ac_dialogmanager_npc (delegate Custom|OnDialogCompleted)))

(event EventInteractwith
  (params (Player :type BP%20Player%20Object%20Reference))
  ;[1 1 1] Interact
  (|CallParentFunction Player))

(event EventBeginPlay
  (|CallParentFunction)
  (Utilities|FlowControl|Sequence
    (:then_0
      (Variables|Default|SetCanLookPlayer false)
      (bind _aswbp_npcdialog (Utilities|Casting|CastToWBP_NPCDialog (UserInterface|GetWidget (Variables|Default|GetDialogWidgetComponent))))
      (bind _output_get (Variables|Default|SetDialogWidgetActor _aswbp_npcdialog))
      (Default|SetOwner _output_get self))
    (:then_1
      (CallFunction|InitStartTalkingButton)
      (Default|Init (Variables|Default|GetAC_DialogManager_NPC))
      (CallFunction|BindDialogEvents))))

(event EventCancelInteract
  (params (Player :type BP%20Player%20Object%20Reference))
  ;[1 1 1] Interact
  (|CallParentFunction Player))

(fn ConstructionScript)