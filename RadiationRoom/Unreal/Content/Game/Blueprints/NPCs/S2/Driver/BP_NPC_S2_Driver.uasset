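; Driver NPC for the car accident scenario, who moves to a safe point and then reports as safe.
; Finishing the first conversation triggers the sit-to-stand and walking flags, and player interaction is blocked while walking.
; StartWalking has its AI controller send it to the destination point.
; StopWalking switches to idle, looks at the player, advances the dialogue, marks the driver protected and fires the NPC-is-safe event.
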(event Custom|StartWalking
  (bind _ascontroller_npc_car_accident_driver (Utilities|Casting|CastToController_NPC_CarAccident_Driver (AI|GetAIController self)))
  (Default|GotoSafePoint _ascontroller_npc_car_accident_driver (Variables|Default|GetDestinationPoint)))

(event Custom|StopWalking
  (Variables|Default|SetWalking false)
  (Variables|Animation|SetWalkToIdle true)
  (CallFunction|LookatPlayer)
  (Variables|Default|SetCanLookPlayer true)
  (Default|NextConversation (Variables|Default|GetAC_DialogManager_NPC))
  (Variables|Default|SetProtected true)
  (Default|CallEDNPCIsSafe))

(event EventInteractwith
  (params (Player :type BP%20Player%20Object%20Reference))
  (if (not (Variables|Default|GetWalking))
    (|CallParentFunction Player)))

(event EventConversationFinished
  (params (Conversation%20ID :type Name :default "None"))
  (|CallParentFunction Conversation%20ID)
  (switch name Conversation%20ID
    (:0
      (if (not (Variables|Animation|GetSitToStand))
        (Variables|Animation|SetSitToStand true)
        (Variables|Default|SetWalking true)))))

(fn ConstructionScript
  (|CallParentFunction))