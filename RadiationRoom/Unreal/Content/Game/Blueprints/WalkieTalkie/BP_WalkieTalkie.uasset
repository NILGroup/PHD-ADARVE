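; Interactable walkie-talkie item through which the player makes initial and final report conversations in a scenario.
; Registers with the gameplay manager and takes conversation data from the game instance, binding a callback if the scenario has not yet initiated.
; Widget buttons start conversations in the dialog manager component, which is given a typewriter effect component.
; When one finishes, it hides the widget after a delay and broadcasts that report's completion.
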(event Custom|BindEvents
  (bind _widgetactor (Variables|Default|GetWidgetActor))
  (EventDispatchers|BindEventtoEDInitialReportButtonClicked _widgetactor (delegate Custom|OnInitialReportButtonClicked))
  (EventDispatchers|BindEventtoEDFinalReportButtonClicked _widgetactor (delegate Custom|OnFinalReportButtonClicked))
  (EventDispatchers|BindEventtoConversationFinished (Variables|Default|GetAC_WalkieDialogManager) (delegate Custom|OnConversationFinished)))

(event Custom|OnConversationFinished
  (params (Walkie%20Conversation%20Type :type E_WalkieConversationType%20Enum :default "NewEnumerator0"))
  (Utilities|FlowControl|Delay 1.0)
  (Development|SetHiddeninGame (Variables|Default|GetWidgetComponent) true false)
  (switch Utilities|FlowControl|Switch|SwitchonE_WalkieConversationType Walkie%20Conversation%20Type
    (:NewEnumerator1
      (Default|CallEDInitialReportCompleted)
      (Variables|Default|SetInitialReportCompleted true))
    (:NewEnumerator2
      (Default|CallEDFinalReportCompleted)
      (Variables|Default|SetFinalReportCompleted true))))

(event Custom|SetInitialConditions
  (params (InitialReportCompleted :type Boolean) (FinalReportCompleted :type Boolean))
  ;[1 1 1] Set Initial Conditions
  (Variables|Default|SetInitialReportCompleted InitialReportCompleted)
  (Variables|Default|SetFinalReportCompleted FinalReportCompleted))

(event Custom|OnFinalReportButtonClicked
  (Default|StartConversation (Variables|Default|GetAC_WalkieDialogManager) "NewEnumerator2"))

(event Custom|OnInitialReportButtonClicked
  (Default|StartConversation (Variables|Default|GetAC_WalkieDialogManager) "NewEnumerator1"))

(event Custom|Init
  (CallFunction|SetWalkieConversationData (Variables|/Game/Game/Blueprints/RR_GameInstance.RR_GameInstance_C|GetWalkieConversation (CallFunction|GetMyGameInstance)))
  (CallFunction|BindEvents))

(event Custom|SetWalkieConversationData
  (params (Walkie%20Conversation%20Data :type Data%20Table%20Object%20Reference))
  ;[1 1 1] Set Initial Conditions
  (Utilities|IsValid Walkie%20Conversation%20Data
    (:Is%20Valid
      (Default|SetWalkieConversationData (Variables|Default|GetAC_WalkieDialogManager) Walkie%20Conversation%20Data))))

(event Custom|SetInitialReportCompleted
  (params (InitialReportCompleted :type Boolean))
  ;[1 1 1] Set Initial Conditions
  (Variables|Default|SetInitialReportCompleted InitialReportCompleted)
  (Default|EnableSpecificButtons (Variables|Default|GetWidgetActor) (not (Variables|Default|GetInitialReportCompleted)) (not (Variables|Default|GetFinalReportCompleted))))

(event Custom|SetFinalReportCompleted
  (params (FinalReportCompleted :type Boolean))
  ;[1 1 1] Set Initial Conditions
  (Variables|Default|SetFinalReportCompleted FinalReportCompleted)
  (Default|EnableSpecificButtons (Variables|Default|GetWidgetActor) (not (Variables|Default|GetInitialReportCompleted)) (not (Variables|Default|GetFinalReportCompleted))))

(event EventBeginPlay
  (bind _gameplaymanager (CallFunction|GetMyGameplayManager))
  (|CallParentFunction)
  (Utilities|FlowControl|Sequence
    (:then_0
      (bind _aswbp_walkie_talkie (Utilities|Casting|CastToWBP_WalkieTalkie (UserInterface|GetWidget (Variables|Default|GetWidgetComponent))))
      (bind _output_get (Variables|Default|SetWidgetActor _aswbp_walkie_talkie))
      (Default|SetOwner _output_get self)
      (Default|SetWidgetComponent (Variables|Default|GetAC_WalkieDialogManager) (Variables|Default|GetWidgetComponent) (Variables|Default|GetWidgetActor))
      (Default|SetTypewriterComponent (Variables|Default|GetAC_WalkieDialogManager) (Variables|Default|GetAC_TypewritterEffect))
      (Development|SetHiddeninGame (Variables|Default|GetWidgetComponent) true false))
    (:then_1
      (Utilities|IsValid _gameplaymanager
        (:Is%20Valid
          (Default|AddItemtoGameManagerImportantList _gameplaymanager (Variables|Default|GetItemType) self))))
    (:then_2
      (if (Variables|/Game/Game/Blueprints/RR_GameInstance.RR_GameInstance_C|GetIsScenarioAlreadyInitiated? (CallFunction|GetMyGameInstance))
        (CallFunction|Init)
        (else
          (EventDispatchers|BindEventtoEDScenarioInitiated (CallFunction|GetMyGameInstance) (delegate Custom|Init)))))
    (:then_3
      (CallFunction|SetWalkieConversationData (Variables|/Game/Game/Blueprints/RR_GameInstance.RR_GameInstance_C|GetWalkieConversation (CallFunction|GetMyGameInstance)))
      (CallFunction|BindEvents))))

(event EventCancelInteract
  (params (Player :type BP%20Player%20Object%20Reference) (Hand :type EControllerHand%20Enum :default "Left"))
  (|CallParentFunction Player Hand)
  (Default|CancelInteract (Variables|Default|GetAC_WalkieDialogManager)))

(event EventInteractwith
  (params (Player :type BP%20Player%20Object%20Reference) (Hand :type EControllerHand%20Enum :default "Left"))
  (|CallParentFunction Player Hand)
  (if (Variables|Default|GetCanShowDialogBox)
    (Default|Interactwith (Variables|Default|GetAC_WalkieDialogManager))))

(fn ConstructionScript
  (|CallParentFunction))