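; Game Instance for a VR experiment game, holding session-wide player, scenario, gameplay-step and database state, announced through event dispatchers.
; Scenario init loads control variables from DataTables, passes walkie-talkie conversations to their actors and positions the player; lookups prefer scenario values over those loaded at startup.
; It also sends user details to the database manager, opens levels and provides logging.
; Player-set notification is briefly delayed so GameplayManager can bind first.
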(event Custom|SetGameplayStepsData
  (params (GameplayStepsData :type Array%20of%20F%20Gameplay%20Step%20Data%20Structures))
  (Utilities|Array|Clear (Variables|Gameplay|GetCurrentGameplayStepsData))
  (Variables|Gameplay|SetCurrentGameplayStepsData GameplayStepsData))

(event Custom|SetCurrentDataBase
  (params (DataBaseManager :type BP%20Data%20Base%20Manager%20Object%20Reference))
  (Variables|Default|SetDatabase%20Manager DataBaseManager)
  (CallFunction|SendUsertoDB)
  (Default|CallEDDatabaseSetted))

(event Custom|CloseDatabase
  (bind _database_manager (Variables|Default|GetDatabase%20Manager)
    (:then
      (EventDispatchers|BindEventtoEDDatabaseClosed _database_manager (delegate Custom|DatabaseClosed))
      (Default|StopandCloseDatabase _database_manager))
    (:else)))

(event Custom|DatabaseClosed
  (Default|CallEDDatabaseClosed))

(event EventInit
  (Utilities|FlowControl|Sequence
    (:then_0
      (CallFunction|SetDefaultVars)
      (Default|CallEDDefaultVarsSetted))
    (:then_1
      (bind _controlvars (CallFunction|GetControlVarsfromDataTable (CallFunction|GetCurrentScenarioControlVars)))
      (Variables|ControlVar|SetControlVars _controlvars)
      (Variables|Default|SetCurrent%20VR%20HMD%20Name (Class|HeadMountedDisplayFunctionLibrary|GetHMDDeviceName)))))

(event Custom|Log
  (params (LogType :type E_LogMessageType%20Enum :default "NewEnumerator0") (Text :type Text) (Show%20In%20Screen :type Boolean))
  (switch Utilities|FlowControl|Switch|SwitchonE_LogMessageType LogType
    (:NewEnumerator1
      (Development|PrintString (Utilities|String|ToString(Text) (Utilities|Text|FormatText "Debug: {text}" Text)) Show%20In%20Screen))
    (:NewEnumerator2
      (Development|PrintString (Utilities|String|ToString(Text) (Utilities|Text|FormatText "Warning: {text}" Text)) Show%20In%20Screen))
    (:NewEnumerator3
      (Development|PrintString (Utilities|String|ToString(Text) (Utilities|Text|FormatText "Error: {text}" Text)) Show%20In%20Screen))))

(event Custom|SetCurrentScenarioData
  (params (Current%20Scenario%20Data :type Data%20Table%20Row%20Handle%20Structure))
  (Variables|LevelInfo|SetCurrent%20Scenario%20Data Current%20Scenario%20Data)
  (Default|CallEDScenarioSelected))

(event Custom|InitScenario
  (params (Current%20Scenario%20Data :type Data%20Table%20Row%20Handle%20Structure) (Player%20Start%20Location :type Vector))
  (CallFunction|SetCurrentScenarioData Current%20Scenario%20Data)
  (CallFunction|InitNewLevelConditions (CallFunction|GetCurrentScenarioControlVars) (CallFunction|GetCurrentScenarioWalkieConversation) (CallFunction|GetCurrentScenarioActiveTutorialItems) Player%20Start%20Location)
  (Default|CallEDScenarioInitiated)
  (Variables|Default|SetIsScenarioAlreadyInitiated? true))

(event Custom|InitNewLevelConditions
  (params (ControlVarsDataTable :type Data%20Table%20Object%20Reference%20%28by%20ref%29) (WalkieConversationDataTable :type Data%20Table%20Object%20Reference) (Active%20TutorialItems%20DataTable :type Data%20Table%20Object%20Reference) (Player%20Location :type Vector))
  (Utilities|FlowControl|Sequence
    (:then_0
      (Utilities|IsValid ControlVarsDataTable
        (:Is%20Valid
          (Variables|ControlVar|SetControlVars%20DataTable ControlVarsDataTable)
          (Utilities|Map|Clear (Variables|ControlVar|GetScenarioControlVars))
          (bind _controlvars (CallFunction|GetControlVarsfromDataTable (Variables|ControlVar|GetControlVars%20DataTable)))
          (Variables|ControlVar|SetScenarioControlVars _controlvars))))
    (:then_1
      (bind _output_get (Variables|Default|SetWalkieConversation WalkieConversationDataTable))
      (Utilities|IsValid _output_get
        (:Is%20Valid
          (bind _outactors (Actor|GetAllActorsOfClass "/Game/Game/Blueprints/WalkieTalkie/BP_WalkieTalkie.BP_WalkieTalkie_C"))
          (for _array_element _outactors
            (Default|SetWalkieConversationData _array_element (Variables|Default|GetWalkieConversation))))))
    (:then_3
      (CallFunction|SetPlayerStartPosition Player%20Location))))

(event EventLoadNextStreamingLevel
  ;[1 1 1] Load and Open Scenarios
  (Variables|Default|SetIsScenarioAlreadyInitiated? false)
  (Variables|LevelInfo|SetPrevious%20Level%20to%20Unload (CallFunction|GetCurrentScenarioName)))

(event EventOpenNextStreamingLevel
  ;[1 1 1] Load and Open Scenarios
  (Game|OpenLevel(byName) (Variables|LevelInfo|GetLevel%20to%20Load)))

(event Custom|SetTutorialType)

(event Custom|SetDefaultVars
  (bind _returnvalue (Utilities|GetDataTableRow "/Game/Game/DataStructures/ControlVars/DT_DefaultVars.DT_DefaultVars" "Data")
    (:then
      (Variables|Default|SetDeveloping? (.Developing (Utilities|Struct|BreakF_DefaultVars _returnvalue))))))

(event Custom|SendUserToDB
  (bind _userid (Variables|PlayerData|GetUserID))
  (if (not (Utilities|Array|IsEmpty _userid))
    (bind _database_manager (Variables|Default|GetDatabase%20Manager)
      (:then
        (Default|SendUsertoDB _database_manager (Utilities|Struct|MakeF_User _userid (Variables|PlayerData|GetUserGroupType) (Variables|PlayerData|GetExperimentID) (Variables|PlayerData|GetUserHMDType) (Math|DateTime|Now))))
      (:else))))

(event Custom|SetPlayerStartPosition
  (params (Location :type Vector))
  (bind _currentplayer (Variables|Player|GetCurrentPlayer)
    (:then
      (Transformation|SetWorldLocation (Variables|/Script/Engine.Character|GetCapsuleComponent _currentplayer) Location false false)
      (Default|InitPlayerConditions (Variables|Player|GetCurrentPlayer)))
    (:else)))

(event Custom|SetPlayer
  (params (Player :type BP%20Player%20Object%20Reference))
  (Variables|Player|SetCurrentPlayer Player)
  (Utilities|FlowControl|Delay 0.2) ; Se añade un pequeño delay para darle tiempo al GameplayManager a crearse y pueda escuchar el callback de ED Player Setted
  (Default|CallEDPlayerSetted))

(fn GetControlVarsfromDataTable
  (params (ControlVars%20DataTable :type Data%20Table%20Object%20Reference))
  (bind _outrownames (DataTable|GetDataTableRowNames ControlVars%20DataTable))
  (for _array_element _outrownames
    (bind _returnvalue (Utilities|GetDataTableRow ControlVars%20DataTable _array_element)
      (:then
        (Utilities|Map|Add (LocalVariables|GetAuxControlVars) (.ControlVarType (Utilities|Struct|BreakF_ControlVarData _returnvalue)) (.State (Utilities|Struct|BreakF_ControlVarData _returnvalue))))))
  (return (LocalVariables|GetAuxControlVars)))

(fn GetControlVar
  (params (ControlVar%20Type :type E_ControlVars%20Enum :default "NewEnumerator0"))
  (bind _scenariocontrolvars (Variables|ControlVar|GetScenarioControlVars))
  (bind (_value _returnvalue) (Utilities|Map|Find _scenariocontrolvars ControlVar%20Type))
  (if _returnvalue
    (return _value)
    (else
      (return (.Value (Utilities|Map|Find (Variables|ControlVar|GetControlVars) ControlVar%20Type))))))

(fn GetDataBaseMainInfoEvent
  (Variables|Player|GetCurrentPlayer
    (:then
      (return (Utilities|Struct|MakeF_MainInfoEvent (Variables|PlayerData|GetUserID) (Variables|PlayerData|GetExperimentID) (CallFunction|GetCurrentScenarioId))))
    (:else
      (return ""))))

(fn GetActiveTutorialItemIDsfromDataTable
  (bind _outrownames (DataTable|GetDataTableRowNames (Variables|Tutorial|GetActive%20TutorialItemsIDs%20DataTable)))
  (for _array_element _outrownames
    (bind _returnvalue (Utilities|GetDataTableRow (Variables|Tutorial|GetActive%20TutorialItemsIDs%20DataTable) _array_element)
      (:then
        (if (.Active (Utilities|Struct|BreakF_TutorialItemPerScenario _returnvalue))
          (Utilities|Array|Add (Variables|Tutorial|GetActiveTutorialItemIDs) (.Id (Utilities|Struct|BreakF_TutorialItemPerScenario _returnvalue))))))))