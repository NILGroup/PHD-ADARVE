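; BP_LevelCreator procedurally builds a rectangular room from a tiled floor and perimeter walls in its construction script.
; It adds separate Instanced Static Mesh components for floor and walls, then multiplies room size by scale factors to get tile counts.
; Helper functions generate a floor grid and four wall rows, two rotated 90 degrees, all spaced by the floor mesh's local bounds maximum, and feed them in as instances.
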(event EventBeginPlay)

(event Collision|EventActorBeginOverlap
  (params (OtherActor :type Actor%20Object%20Reference)))

(event EventTick
  (params (DeltaSeconds :type Float%20%28single-precision%29)))

(fn ConstructionScript
  (CallFunction|CreateLevel))

(fn CreateLevel
  (CallFunction|CreateInstances)
  (RoomFunctions|CreateRoom))

(fn CreateInstances
  (Utilities|FlowControl|Sequence
    (:then_0
      (Utilities|FlowControl|Sequence
        (:then_0
          (bind _returnvalue (AddComponent|AddInstancedStaticMeshComponent false))
          (Variables|Meshes|SetISM_RoomFloor _returnvalue))
        (:then_1
          (bind _returnvalue_2 (AddComponent|AddInstancedStaticMeshComponent false))
          (Variables|Meshes|SetISM_RoomWall _returnvalue_2))))))

(fn CreateRoom
  (Utilities|FlowControl|Sequence
    (:then_0
      (Variables|RoomSettings|SetRoom%20Scaled%20Size%20X (* (Variables|RoomSettings|GetRoom%20Size%20X) (Variables|Default|GetSize%20Scale%20X)))
      (Variables|RoomSettings|SetRoom%20Scaled%20Size%20Y (* (Variables|RoomSettings|GetRoom%20Size%20Y) (Variables|Default|GetSize%20Scale%20Y))))
    (:then_1
      (bind _transforms (RoomFunctions|MakeRoomFloorTransforms))
      (Components|InstancedStaticMesh|AddInstances (Variables|Meshes|GetISM_RoomFloor) _transforms false false true))
    (:then_2
      (bind _transforms_2 (RoomFunctions|MakeRoomWallTransforms))
      (Components|InstancedStaticMesh|AddInstances (Variables|Meshes|GetISM_RoomWall) _transforms_2 false false true))))

(fn MakeRoomFloorTransforms
  (bind _ism_roomfloor (Variables|Meshes|GetISM_RoomFloor))
  (bind _max (Components|StaticMesh|GetLocalBounds _ism_roomfloor))
  (Utilities|FlowControl|Sequence
    (:then_0
      (LocalVariables|SetFloor%20Size%20X (.x _max))
      (LocalVariables|SetFloor%20Size%20Y (.y _max)))
    (:then_1
      (for _index (range 0 (- (Variables|RoomSettings|GetRoom%20Scaled%20Size%20X) 1))
        (for _index_2 (range 0 (- (Variables|RoomSettings|GetRoom%20Scaled%20Size%20Y) 1))
          (Utilities|Array|Add (LocalVariables|GetFloorTransforms) (Math|Transform|MakeTransform (Math|Vector|MakeVector (* _index (LocalVariables|GetFloor%20Size%20X)) (* _index_2 (LocalVariables|GetFloor%20Size%20Y)) 0.0))))))
    (:then_2
      (return (LocalVariables|GetFloorTransforms)))))

(fn MakeRoomWallTransforms
  (bind _ism_roomfloor (Variables|Meshes|GetISM_RoomFloor))
  (bind _max (Components|StaticMesh|GetLocalBounds _ism_roomfloor))
  (Utilities|FlowControl|Sequence
    (:then_0
      (LocalVariables|SetFloor%20Size%20X (.x _max))
      (LocalVariables|SetFloor%20Size%20Y (.y _max)))
    (:then_1
      (for _index (range 0 1)
        (for _index_2 (range 0 (- (Variables|RoomSettings|GetRoom%20Scaled%20Size%20X) 1))
          (Utilities|Array|Add (LocalVariables|GetWallTransforms) (Math|Transform|MakeTransform (Math|Vector|MakeVector (* _index_2 (LocalVariables|GetFloor%20Size%20X)) (* _index (Variables|RoomSettings|GetRoom%20Scaled%20Size%20Y) (LocalVariables|GetFloor%20Size%20Y)) 0.0))))))
    (:then_2
      (for _index_3 (range 0 1)
        (for _index_4 (range 0 (- (Variables|RoomSettings|GetRoom%20Scaled%20Size%20Y) 1))
          (Utilities|Array|Add (LocalVariables|GetWallTransforms) (Math|Transform|MakeTransform (Math|Vector|MakeVector (* _index_3 (Variables|RoomSettings|GetRoom%20Scaled%20Size%20X) (LocalVariables|GetFloor%20Size%20X)) (* _index_4 (LocalVariables|GetFloor%20Size%20Y)) 0.0) "0.000000,90.000000,0.000000")))))
    (:then_3
      (return (LocalVariables|GetWallTransforms)))))