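; Gameplay manager for assessment scenarios that starts with the quest list panels and scenario description panel hidden.
; On BeginPlay it finds those actors, deactivates the description panel's quest list and still fills both with tracking descriptions from QuestDataTable.
; StartScenario extends the parent by showing StartTuddy.
; CompleteQuest runs the parent logic, then forwards the quest ID to every panel.
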(event Custom|FindQuestListWidgets
  (Utilities|FlowControl|Sequence
    (:then_0
      (bind _outactors (Actor|GetAllActorsOfClass "/Game/Game/Blueprints/Widgets/QuestPanels/BP_QuestListPanel.BP_QuestListPanel_C"))
      (bind _output_get (Variables|Default|SetQuestListWidget _outactors))
      (for _array_element _output_get
        (Rendering|SetActorHiddenInGame _array_element true)))
    (:then_1
      (bind _returnvalue (Actor|GetActorOfClass "/Game/Game/Blueprints/Widgets/QuestPanels/BP_ScenarioDescriptionActor.BP_ScenarioDescriptionActor_C"))
      (Variables|Default|SetScenarioDescriptionPanel _returnvalue)
      (bind _scenariodescriptionpanel (Variables|Default|GetScenarioDescriptionPanel)
        (:then
          (Rendering|SetActorHiddenInGame _scenariodescriptionpanel true)
          (Default|ActivateQuestList _scenariodescriptionpanel false))
        (:else)))))

(event EventBeginPlay
  (|CallParentFunction)
  (CallFunction|FindQuestListWidgets)
  (CallFunction|SetQuestListinPanel))

(event EventCompleteQuest
  (params (QuestID :type Name :default "None"))
  (|CallParentFunction QuestID)
  (Utilities|FlowControl|Sequence
    (:then_0
      (for _array_element (Variables|Default|GetQuestListWidget)
        (Default|CompleteQuest _array_element QuestID)))
    (:then_1
      (bind _scenariodescriptionpanel (Variables|Default|GetScenarioDescriptionPanel)
        (:then
          (Default|CompleteQuest _scenariodescriptionpanel QuestID))
        (:else)))))

(event EventStartScenario
  (|CallParentFunction)
  (Default|Show (Variables|Default|GetStartTuddy)))

(fn ConstructionScript
  (|CallParentFunction))

(fn SetQuestListinPanel
  (bind _quests (LocalVariables|GetQuests))
  (bind _outrownames (DataTable|GetDataTableRowNames (Variables|Default|GetQuest%20Data%20Table)))
  (for _array_element _outrownames
    (bind _returnvalue (Utilities|GetDataTableRow (Variables|Default|GetQuest%20Data%20Table) _array_element)
      (:then
        (Utilities|Map|Add (LocalVariables|GetQuests) _array_element (.TrackingDescription (Utilities|Struct|BreakF_QuestData _returnvalue))))))
  (Utilities|FlowControl|Sequence
    (:then_0
      (for _array_element_2 (Variables|Default|GetQuestListWidget)
        (Default|SetQuestList _array_element_2 _quests)))
    (:then_1
      (bind _scenariodescriptionpanel (Variables|Default|GetScenarioDescriptionPanel)
        (:then
          (Default|SetQuestList _scenariodescriptionpanel _quests))
        (:else)))))