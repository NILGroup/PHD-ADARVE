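; BP_GameplayManager_T2 is a gameplay manager for scenario T2 that drives Tuddy's opening and closing dialogs.
; It extends a parent manager, calling the parent's begin play, start and binding events before adding its own logic.
; Starting the scenario plays dialog T2001 on the start Tuddy.
; When the player overlaps the end trigger and gameplay is completed, the end Tuddy plays dialog T2002.
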(event Custom|OnActorOverlapEndTrigger
  (params (OverlappedActor :type Actor%20Object%20Reference) (OtherActor :type Actor%20Object%20Reference))
  (if (== OtherActor (CallFunction|GetMyPlayer))
    (if (CallFunction|IsGameplayCompleted)
      (Default|StartNewDialog (Variables|/Game/Game/Blueprints/Tutorial/BP_TutorialBuddy.BP_TutorialBuddy_C|GetAC_DialogManager_Tuddy (Variables|Default|GetEndTuddy)) "T2002"))))

(event EventBindPlayerActions
  (|CallParentFunction)
  (Collision|BindEventtoOnActorBeginOverlap (Variables|Default|GetEndTrigger) (delegate Custom|OnActorOverlapEndTrigger)))

(event EventBeginPlay
  (|CallParentFunction))

(event EventStartScenario
  (|CallParentFunction)
  (Default|StartNewDialog (Variables|/Game/Game/Blueprints/Tutorial/BP_TutorialBuddy.BP_TutorialBuddy_C|GetAC_DialogManager_Tuddy (Variables|Default|GetStartTuddy)) "T2001"))

(fn ConstructionScript)