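; Gameplay manager for the T1 tutorial scenario, extending a parent manager and running the flow from Tuddy's intro dialog to gameplay end.
; BeginPlay passes place-point managers and the NPC to their quests.
; After the intro dialog and welcome countdown, it teleports the player and starts the first quest and tutorial display, which advances on each completion.
; Once all quests finish, an end trigger starts Tuddy's closing dialog, then a goodbye countdown ends gameplay.
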(event EventBeginPlay
  (|CallParentFunction)
  (Utilities|FlowControl|Sequence
    (:then_0
      (Variables|Default|SetStartQuestAllowed false)
      (Rendering|SetActorHiddenInGame (Variables|Default|GetGoodbyeWidget) true))
    (:then_1
      (Utilities|FlowControl|Sequence
        (:then_0
          (bind _asbp_quest_t1_pla (Utilities|Casting|CastToBP_Quest_T1_PLA (.Value (Utilities|Map|Find (Variables|Default|GetQuestActorList) "T1004"))))
          (Variables|/Game/Game/Blueprints/Gameplay/Quest/T1/BP_Quest_T1_PLA.BP_Quest_T1_PLA_C|SetPlacePointManagers _asbp_quest_t1_pla (Variables|Default|GetPlacePointManagers)))
        (:then_1
          (bind _asbp_quest_t1_npc (Utilities|Casting|CastToBP_Quest_T1_NPC (.Value (Utilities|Map|Find (Variables|Default|GetQuestActorList) "T1005"))))
          (Variables|/Game/Game/Blueprints/Gameplay/Quest/T1/BP_Quest_T1_NPC.BP_Quest_T1_NPC_C|SetNPC _asbp_quest_t1_npc (Variables|Default|GetNPC)))))))

(event EventStartScenario
  (bind _starttuddy (Variables|Tuddy|GetStartTuddy))
  (|CallParentFunction)
  (Default|Show _starttuddy)
  (Utilities|FlowControl|Delay 0.5)
  (Default|StartNewDialogbyID (Variables|/Game/Game/Blueprints/Tutorial/BP_TutorialBuddy.BP_TutorialBuddy_C|GetAC_TuddyDialogManager _starttuddy) "T1001"))

(event EventCompleteQuest
  (params (QuestID :type Name :default "None"))
  (|CallParentFunction QuestID)
  (Variables|Default|SetStartQuestAllowed false)
  (Default|NextDisplay (Variables|Default|GetTutorialDisplayManager))
  (if (CallFunction|IsGameplayCompleted)
    (Utilities|FlowControl|Delay 1.0)
    (Default|Show (Variables|Tuddy|GetEndTuddy))
    (Rendering|SetActorHiddenInGame (Variables|Default|GetGoodbyeWidget) false)))

(event Custom|OnGoodbyeCountdownCompleted
  (CallFunction|EndGameplay))

(event Custom|OnStartTuddyDialogCompleted
  (params (CurrentTuddyDialogType :type E_TuddyDialogLinesType%20Enum :default "NewEnumerator0") (CurrentExtraLineType :type E_TuddyExtraLineTypes%20Enum :default "NewEnumerator1") (DialogID :type Name))
  (bind _welcomewidget (Variables|Default|GetWelcomeWidget))
  (Default|Hide (Variables|Tuddy|GetStartTuddy))
  (Rendering|SetActorHiddenInGame (Variables|Default|GetWelcomeWidget) false)
  (Default|StartCountdown _welcomewidget)
  (EventDispatchers|BindEventtoEDCountdownEnded _welcomewidget (delegate Custom|OnWelcomeCountdownCompleted)))

(event Custom|OnEndTuddyDialogCompleted
  (params (CurrentTuddyDialogType :type E_TuddyDialogLinesType%20Enum :default "NewEnumerator0") (CurrentExtraLineType :type E_TuddyExtraLineTypes%20Enum :default "NewEnumerator1") (DialogID :type Name))
  (bind _goodbyewidget (Variables|Default|GetGoodbyeWidget))
  (Default|Hide (Variables|Tuddy|GetEndTuddy))
  (Rendering|SetActorHiddenInGame (Variables|Default|GetGoodbyeWidget) false)
  (Default|StartCountdown _goodbyewidget)
  (EventDispatchers|BindEventtoEDCountdownEnded _goodbyewidget (delegate Custom|OnGoodbyeCountdownCompleted)))

(event Custom|OnWelcomeCountdownCompleted
  (Transformation|SetActorLocation (CallFunction|GetMyPlayer) (Transformation|GetActorLocation (Variables|Default|GetInitialTeleportPoint)) false true)
  (CallFunction|SetCurrentQuest "T1002")
  (Default|StartFirstDisplay (Variables|Default|GetTutorialDisplayManager)))

(event EventBindTuddyActions
  (|CallParentFunction)
  (EventDispatchers|BindEventtoEDDialogCompleted (Variables|/Game/Game/Blueprints/Tutorial/BP_TutorialBuddy.BP_TutorialBuddy_C|GetAC_TuddyDialogManager (Variables|Tuddy|GetStartTuddy)) (delegate Custom|OnStartTuddyDialogCompleted))
  (EventDispatchers|BindEventtoEDDialogCompleted (Variables|/Game/Game/Blueprints/Tutorial/BP_TutorialBuddy.BP_TutorialBuddy_C|GetAC_TuddyDialogManager (Variables|Tuddy|GetEndTuddy)) (delegate Custom|OnEndTuddyDialogCompleted)))

(event Custom|OnActorOverlapEndTrigger
  (params (OverlappedActor :type Actor%20Object%20Reference) (OtherActor :type Actor%20Object%20Reference))
  (if (== OtherActor (CallFunction|GetMyPlayer))
    (if (CallFunction|IsGameplayCompleted)
      (Default|StartNewDialogbyID (Variables|/Game/Game/Blueprints/Tutorial/BP_TutorialBuddy.BP_TutorialBuddy_C|GetAC_TuddyDialogManager (Variables|Tuddy|GetEndTuddy)) "T1002"))))

(event EventBindPlayerActions
  (|CallParentFunction)
  (Collision|BindEventtoOnActorBeginOverlap (Variables|Default|GetEndTrigger) (delegate Custom|OnActorOverlapEndTrigger)))

(fn ConstructionScript)