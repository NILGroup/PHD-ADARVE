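; Scenario gameplay manager that runs a quest sequence and loads the next level or quits when gameplay ends.
; On BeginPlay it registers with the GameInstance and builds BP_Quest objects from a data table.
; Starting a quest broadcasts the change; completing one updates quest panels and the scenario description, while a cheat event completes and advances.
; Scenario start and finish are logged to the database; player, item, place-point, NPC and Tuddy bindings are empty stubs.
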(event Custom|BindTuddyActions)

(event Custom|BindGameInstanceActions
  (EventDispatchers|AssignEDDatabaseClosed (CallFunction|GetMyGameInstance) (delegate Custom|OnDatabaseClosed))
  (EventDispatchers|BindEventtoEDPlayerSetted (CallFunction|GetMyGameInstance) (delegate Custom|OnGameInstancePlayerSetted)))

(event Custom|BindNPCActions)

(event Custom|StartScenario
  (CallFunction|SendStartEventtoDB))

(event Custom|AddItemToGameManagerImportantList
  (params (ItemType :type E_ItemType%20Enum :default "NewEnumerator2") (Actor :type Actor%20Object%20Reference)))

(event Custom|BindPlacePointsActions)

(event Custom|CompleteQuest
  (params (QuestID :type Name))
  (Utilities|FlowControl|Sequence
    (:then_0
      (Default|CompleteQuest (.Value (Utilities|Map|Find (Variables|Quests|GetQuestActorList) QuestID)))
      (for _array_element (Variables|Quests|GetQuestListWidget)
        (Default|CompleteQuest _array_element QuestID)))
    (:then_1
      (bind _returnvalue (Actor|GetActorOfClass "/Game/Game/Blueprints/Widgets/QuestPanels/BP_ScenarioDescriptionActor.BP_ScenarioDescriptionActor_C"))
      (Utilities|IsValid _returnvalue
        (:Is%20Valid
          (bind _descriptionwidget (Variables|/Game/Game/Blueprints/Widgets/QuestPanels/BP_ScenarioDescriptionActor.BP_ScenarioDescriptionActor_C|GetDescriptionWidget _returnvalue)
            (:then
              (Default|CompleteTask _descriptionwidget QuestID))
            (:else)))))))

(event Custom|SendFinishEventToDB
  (CallFunction|SendQuesttoDatabase "00002" "NewEnumerator3"))

(event Custom|OnGameInstancePlayerSetted
  (CallFunction|BindPlayerActions))

(event Custom|LoadNextLevel
  (bind (_exit _next_scenario_data) (CallFunction|GetCurrentScenarioNextData))
  (if _exit
    (Utilities|FlowControl|Delay 0.5)
    (Game|QuitGame 0 "Quit" false)
    (else
      (bind _output_get (Variables|/Game/Game/Blueprints/RR_GameInstance.RR_GameInstance_C|SetLevel%20to%20Load (CallFunction|GetMyGameInstance) (.BPLevelName (Utilities|Struct|BreakF_ScenarioData _next_scenario_data))))
      (Game|OpenLevel(byName) _output_get))))

(event Custom|CreateQuestList
  (bind _outrownames (DataTable|GetDataTableRowNames (Variables|Default|GetQuest%20Data%20Table)))
  (for _array_element _outrownames
    (bind _returnvalue (Utilities|GetDataTableRow (Variables|Default|GetQuest%20Data%20Table) _array_element)
      (:then
        (bind _returnvalue_2 (Game|ConstructObjectfromClass "/Game/Game/Blueprints/Gameplay/Quest/BP_Quest.BP_Quest_C"))
        (Utilities|FlowControl|Sequence
          (:then_0
            (Variables|/Game/Game/Blueprints/Gameplay/Quest/BP_Quest.BP_Quest_C|SetId _returnvalue_2 _array_element)
            (Variables|/Game/Game/Blueprints/Gameplay/Quest/BP_Quest.BP_Quest_C|SetData _returnvalue_2 _returnvalue)
            (Variables|/Game/Game/Blueprints/Gameplay/Quest/BP_Quest.BP_Quest_C|SetGameplayManager _returnvalue_2 self)
            (Variables|/Game/Game/Blueprints/Gameplay/Quest/BP_Quest.BP_Quest_C|SetGameInstance _returnvalue_2 (CallFunction|GetMyGameInstance)))
          (:then_1
            (Utilities|Map|Add (Variables|Quests|GetQuestActorList) _array_element _returnvalue_2)
            (Utilities|Array|AddUnique (Variables|SortQuests|GetSortedQuests) _array_element)))))))

(event Custom|OnDatabaseClosed)

(event Custom|EndGameplay
  (CallFunction|SendFinishEventtoDB)
  (Utilities|FlowControl|Delay 0.5)
  (CallFunction|LoadNextLevel))

(event Custom|CheatButton
  ;[1 1 1] Cheat Button
  (CallFunction|CompleteQuest (Utilities|Array|Get(acopy) (Variables|SortQuests|GetSortedQuests) (Variables|SortQuests|GetCurrentQuestIndex)))
  (if (< (Variables|SortQuests|GetCurrentQuestIndex) (- (Utilities|Array|Length (Variables|SortQuests|GetSortedQuests)) 1))
    (bind _result (Math|Integer|IncrementInt (Variables|SortQuests|GetCurrentQuestIndex))
      (:%20%20
        (CallFunction|SetCurrentQuest (Utilities|Array|Get(acopy) (Variables|SortQuests|GetSortedQuests) _result))))))

(event Custom|BindPlayerActions)

(event Custom|SendStartEventToDB
  (CallFunction|SendQuesttoDatabase "00001" "NewEnumerator3"))

(event Custom|BindItemActions)

(event Custom|SetCurrentQuest
  (params (Quest%20ID :type Name))
  (bind _output_get (Variables|Quests|SetCurrentQuestID Quest%20ID))
  (Default|StartQuest (.Value (Utilities|Map|Find (Variables|Quests|GetQuestActorList) _output_get)))
  (Default|CallEDQuestChanged _output_get))

(event EventBeginPlay
  (Utilities|FlowControl|Sequence
    (:then_0
      (CallFunction|BindGameInstanceActions)
      (CallFunction|BindItemActions)
      (CallFunction|BindPlacePointsActions)
      (CallFunction|BindNPCActions)
      (CallFunction|BindTuddyActions)
      (CallFunction|BindPlayerActions))
    (:then_1
      (Variables|/Game/Game/Blueprints/RR_GameInstance.RR_GameInstance_C|SetGameplayManager (CallFunction|GetMyGameInstance) self)
      (Default|OnGameInstanceDefaultVarsSetted (Variables|Default|GetTutorialManager))
      (bind _outactors (Actor|GetAllActorsOfClass "/Game/Game/Blueprints/Widgets/QuestPanels/BP_QuestListPanel.BP_QuestListPanel_C"))
      (Variables|Quests|SetQuestListWidget _outactors))
    (:then_2
      (CallFunction|CreateQuestList))))

(fn ConstructionScript)

(fn IsCurrentQuest
  (params (QuestID :type Name))
  (return (== QuestID (Variables|Quests|GetCurrentQuestID))))

(fn IsQuestCompleted
  (params (Quest%20ID :type Name))
  (return (Variables|/Game/Game/Blueprints/Gameplay/Quest/BP_Quest.BP_Quest_C|GetCompleted (.Value (Utilities|Map|Find (Variables|Quests|GetQuestActorList) Quest%20ID)))))

(fn IsGameplayCompleted
  (bind _values (Utilities|Map|Values (Variables|Quests|GetQuestActorList)))
  (bind _array_element (Utilities|Array|ForEachLoopwithBreak _values :!label _label)
    (:LoopBody
      (if (Variables|/Game/Game/Blueprints/Gameplay/Quest/BP_Quest.BP_Quest_C|GetCompleted _array_element)
        (LocalVariables|SetGameplayCompleted true)
        (else
          (LocalVariables|SetGameplayCompleted false)
          (goto _label Break))))
    (:Completed
      (return (LocalVariables|GetGameplayCompleted)))))

(fn SendQuesttoDatabase
  (params (Quest%20ID :type Name) (Step%20State :type E_QuestState%20Enum :default "NewEnumerator0"))
  (bind _database_manager (CallFunction|GetMyDataBase))
  (bind _data (Default|GetDataBaseMainInfoEvent (CallFunction|GetMyGameInstance)))
  (Utilities|IsValid _database_manager
    (:Is%20Valid
      (Default|SendGameplayEventtoDB _database_manager (Utilities|Struct|MakeF_GameplayEvent 0 (.user_id (Utilities|Struct|BreakF_MainInfoEvent _data)) (.experiment_id (Utilities|Struct|BreakF_MainInfoEvent _data)) (.scenario_type (Utilities|Struct|BreakF_MainInfoEvent _data)) Quest%20ID Step%20State (Math|DateTime|Now))))))

(fn GetQuestDatabyID
  (params (Quest%20ID :type Name))
  (bind _returnvalue (Utilities|GetDataTableRow (Variables|Default|GetQuest%20Data%20Table) Quest%20ID)
    (:then
      (return _returnvalue))
    (:RowNotFound
      (Default|Log (CallFunction|GetMyGameInstance) "NewEnumerator2" (Utilities|Text|FormatText "La quest {row_name} no existe en la tabla" Quest%20ID) false)
      (return ""))))

(fn IsCurrentQuestandCanStart
  (params (QuestID :type Name))
  (return (and (CallFunction|IsCurrentQuest QuestID) (Variables|Quests|GetCanStartCurrentQuest))))