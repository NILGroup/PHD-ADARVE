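; Scenario 2 gameplay manager that runs a radiological incident training quest line, from tutorial-buddy intro to ending.
; It extends parent binding hooks to turn walkie-talkie, dosimeter, NPC and traffic-cone delegates into guarded quest completions.
; Tuddy dialogs start the description panel and data-table quest list, then remove the small room.
; After the final report, overlapping Tuddy's trigger starts the closing dialog, which ends gameplay.
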(event EventBeginPlay
  (|CallParentFunction)
  (Collision|SetActorEnableCollision (Variables|Default|GetTrafficWall) false))

(event EventAddItemtoGameManagerImportantList
  (params (ItemType :type E_ItemType%20Enum :default "NewEnumerator2") (Actor :type Actor%20Object%20Reference))
  (switch Utilities|FlowControl|Switch|SwitchonE_ItemType ItemType
    (:NewEnumerator1
      (bind _asbp_dosimeter_sabg100 (Utilities|Casting|CastToBP_Dosimeter_SABG100 Actor))
      (CallFunction|BindSAGB100Actions _asbp_dosimeter_sabg100)
      (Utilities|Array|Add (Variables|Dosimeters|GetSABG100List) _asbp_dosimeter_sabg100))
    (:NewEnumerator3
      (bind _asbp_dosimeter_epd (Utilities|Casting|CastToBP_Dosimeter_EPD Actor))
      (CallFunction|BindEPDActions _asbp_dosimeter_epd)
      (Utilities|Array|Add (Variables|Dosimeters|GetEPDList) _asbp_dosimeter_epd))
    (:NewEnumerator5
      (bind _asbp_walkie_talkie (Utilities|Casting|CastToBP_WalkieTalkie Actor))
      (Default|SetInitialConditions _asbp_walkie_talkie (Variables|WalkieReports|GetInitialReportCompleted) (Variables|WalkieReports|GetFinalReportCompleted))
      (CallFunction|BindWalkieTalkieEvents _asbp_walkie_talkie)
      (Utilities|Array|Add (Variables|WalkieReports|GetWalkieTalkieList) _asbp_walkie_talkie))))

(event EventCompleteQuest
  (params (QuestID :type Name :default "None"))
  (|CallParentFunction QuestID)
  (Utilities|FlowControl|Sequence
    (:then_0
      (switch name QuestID
        (:S2009
          (Default|Show (Variables|Tutorial|GetTutorialBuddy))
          (if (Variables|Tutorial|GetPlayerOverlappingTuddyTrigger)
            (Utilities|FlowControl|Delay 0.5)
            (CallFunction|StartEndConversation)))))
    (:then_1
      (if (CallFunction|IsGameplayCompleted)
        _))))

(event EventStartScenario
  (|CallParentFunction)
  (Default|Show (Variables|Tutorial|GetTutorialBuddy))
  (Utilities|FlowControl|Delay 0.5)
  (Default|StartNewDialog (Variables|/Game/Game/Blueprints/Tutorial/BP_TutorialBuddy.BP_TutorialBuddy_C|GetAC_TuddyDialogManager (Variables|Tutorial|GetTutorialBuddy)) "S2001"))

(event EventOnGameInstancePlayerSetted
  (|CallParentFunction))

(event Custom|OnTuddySphereOverlapped
  (params (OverlappedActor :type Actor%20Object%20Reference) (OtherActor :type Actor%20Object%20Reference))
  (if (== OtherActor (CallFunction|GetMyPlayer))
    (Variables|Tutorial|SetPlayerOverlappingTuddyTrigger true)
    (CallFunction|StartEndConversation)))

(event Custom|OnTuddyTriggerEndOverlapped
  (params (OverlappedActor :type Actor%20Object%20Reference) (OtherActor :type Actor%20Object%20Reference))
  (if (== OtherActor (CallFunction|GetMyPlayer))
    (Variables|Tutorial|SetPlayerOverlappingTuddyTrigger false)))

(event EventBindPlayerActions
  (|CallParentFunction)
  (Collision|BindEventtoOnActorBeginOverlap (Variables|Tutorial|GetTuddyTriggerSphere) (delegate Custom|OnTuddySphereOverlapped))
  (Collision|BindEventtoOnActorEndOverlap (Variables|Tutorial|GetTuddyTriggerSphere) (delegate Custom|OnTuddyTriggerEndOverlapped)))

(event Custom|OnDescriptionCompleted
  (Default|SetQuestListVisibility (Variables|Default|GetDescriptionPanel) "Visible")
  (Utilities|FlowControl|Delay 1.0)
  (Default|Show (Variables|Tutorial|GetTutorialBuddy))
  (Utilities|FlowControl|Delay 0.5)
  (Default|StartNewDialog (Variables|/Game/Game/Blueprints/Tutorial/BP_TutorialBuddy.BP_TutorialBuddy_C|GetAC_TuddyDialogManager (Variables|Tutorial|GetTutorialBuddy)) "S2002"))

(event Custom|BindWalkieTalkieEvents
  (params (WalkieTalkie :type BP%20Walkie%20Talkie%20Object%20Reference))
  ;[1 1 1] Walkie-Talkie Actions
  (EventDispatchers|BindEventtoEDInitialReportCompleted WalkieTalkie (delegate Custom|OnWalkieInitialReportCompleted))
  (EventDispatchers|BindEventtoEDFinalReportCompleted WalkieTalkie (delegate Custom|OnWalkieFinalReportCompleted)))

(event Custom|BindSAGB100Actions
  (params (SABG100 :type BP%20Dosimeter%20SABG100%20Object%20Reference))
  ;[1 1 1] SABG-100 Actions
  (EventDispatchers|AssignEDItemRadiationMeasured SABG100 (delegate Custom|OnSABG100ItemRadiationMeasured))
  (EventDispatchers|AssignEDNPCRadiationMeasured SABG100 (delegate Custom|ONSABG100NPCRadiationMeasured)))

(event Custom|OnSABG100ItemRadiationMeasured
  (params (Actor :type BP%20Interact%20Item%20Parent%20Object%20Reference))
  ;[1 1 1] SABG-100 Actions
  (if (not (CallFunction|IsQuestCompleted "S2008"))
    (if (and (== Actor (Variables|Dosimeters|GetRadiactiveItem)) (not (Variables|MeasureRadiation|GetItemRadiationMeasured)))
      (Variables|MeasureRadiation|SetItemRadiationMeasured true)
      (CallFunction|CompleteQuest "S2008"))))

(event Custom|ONSABG100NPCRadiationMeasured
  (params (Actor :type BP%20NPC%20Object%20Reference))
  ;[1 1 1] SABG-100 Actions
  (if (not (CallFunction|IsQuestCompleted "S2007"))
    (Utilities|Casting|CastToBP_NPC_S2_Driver Actor)
    (if (not (Variables|MeasureRadiation|GetNPCRadiationMeasured))
      (Variables|MeasureRadiation|SetNPCRadiationMeasured true)
      (CallFunction|CompleteQuest "S2007"))))

(event Custom|OnWalkieInitialReportCompleted
  ;[1 1 1] Walkie-Talkie Actions
  (if (not (CallFunction|IsQuestCompleted "S2001"))
    (Variables|WalkieReports|SetInitialReportCompleted true)
    (for _array_element (Variables|WalkieReports|GetWalkieTalkieList)
      (Default|SetInitialConditions _array_element (Variables|WalkieReports|GetInitialReportCompleted) (Variables|WalkieReports|GetFinalReportCompleted)))
    (CallFunction|CompleteQuest "S2001")))

(event Custom|OnWalkieFinalReportCompleted
  ;[1 1 1] Walkie-Talkie Actions
  (if (not (CallFunction|IsQuestCompleted "S2009"))
    (Variables|WalkieReports|SetFinalReportCompleted true)
    (for _array_element (Variables|WalkieReports|GetWalkieTalkieList)
      (Default|SetInitialConditions _array_element (Variables|WalkieReports|GetInitialReportCompleted) (Variables|WalkieReports|GetFinalReportCompleted)))
    (CallFunction|CompleteQuest "S2009")))

(event Custom|BindEPDActions
  (params (EPD :type BP%20Dosimeter%20EPD%20Object%20Reference))
  ;[1 1 1] EPD
  (EventDispatchers|BindEventtoEDInteractionStarted EPD (delegate Custom|OnEPDGrabbed)))

(event Custom|BindDescriptionPanelEvents
  (bind _returnvalue (Actor|GetActorOfClass "/Game/Game/Blueprints/Widgets/QuestPanels/BP_ScenarioDescriptionActor.BP_ScenarioDescriptionActor_C"))
  (Variables|Default|SetDescriptionPanel _returnvalue)
  (bind _descriptionpanel (Variables|Default|GetDescriptionPanel)
    (:then
      (EventDispatchers|BindEventtoEDDescriptionCompleted _descriptionpanel (delegate Custom|OnDescriptionCompleted)))
    (:else
      (Default|Log (CallFunction|GetMyGameInstance) "NewEnumerator2" "Falta el DescriptionPanel" false))))

(event Custom|OnEPDGrabbed
  (params (Actor :type BP%20Interact%20Item%20Parent%20Object%20Reference))
  ;[1 1 1] EPD
  (if (not (CallFunction|IsQuestCompleted "S2002"))
    (CallFunction|CompleteQuest "S2002")))

(event Custom|OnOneTrafficConeHasBeenPlaced
  (params (Item :type BP%20Pickable%20Item%20Object%20Reference) (PlacePoint :type BP%20Place%20Point%20Object%20Reference))
  ;[1 1 1] Place Point Actions
  (if (not (CallFunction|IsQuestCompleted "S2006"))
    (CallFunction|CompleteQuest "S2006")
    (Collision|SetActorEnableCollision (Variables|Default|GetTrafficWall) true)))

(event EventBindItemActions
  (|CallParentFunction)
  (CallFunction|BindDescriptionPanelEvents)
  (CallFunction|BindPlacePointsActions))

(event EventBindPlacePointsActions
  ;[1 1 1] Place Point Actions
  (|CallParentFunction)
  (bind _returnvalue (Actor|GetActorOfClass "/Game/Game/Blueprints/Actors/Items/PlacePoints/BP_PlacePointManager.BP_PlacePointManager_C"))
  (Utilities|IsValid _returnvalue
    (:Is%20Valid
      (EventDispatchers|AssignEDOneItemHasBeenPlaced _returnvalue (delegate Custom|OnOneTrafficConeHasBeenPlaced)))
    (:Is%20Not%20Valid
      (Default|Log (CallFunction|GetMyGameInstance) "NewEnumerator2" "Falta el PlacePointManager de los \"conos de tráfico\"" false))))

(event Custom|BindNPCWitnessActions
  (bind _npc_witness (Variables|NPCs|GetNPC%20Witness)
    (:then
      (EventDispatchers|BindEventtoEDConversationFinished _npc_witness (delegate Custom|OnNPCWitnessConversationFinished)))
    (:else
      (Default|Log (CallFunction|GetMyGameInstance) "NewEnumerator2" "Falta NPC Witness" false))))

(event Custom|BindNPCDriverActions
  (bind _npc_driver (Variables|NPCs|GetNPC%20Driver)
    (:then
      (EventDispatchers|BindEventtoEDConversationFinished _npc_driver (delegate Custom|OnNPCDriverConversationFinished))
      (EventDispatchers|BindEventtoEDNPCProtected _npc_driver (delegate Custom|OnNPCDriverProtected)))
    (:else
      (Default|Log (CallFunction|GetMyGameInstance) "NewEnumerator2" "Falta NPC Driver" false))))

(event Custom|OnNPCWitnessConversationFinished
  (params (ConversationNumber :type Integer))
  (if (not (CallFunction|IsQuestCompleted "S2003"))
    (CallFunction|CompleteQuest "S2003")))

(event Custom|OnNPCDriverConversationFinished
  (params (ConversationNumber :type Integer))
  (switch int ConversationNumber
    (:1
      (if (not (CallFunction|IsQuestCompleted "S2005"))
        (CallFunction|CompleteQuest "S2005")))))

(event Custom|OnNPCDriverProtected
  (if (not (CallFunction|IsQuestCompleted "S2004"))
    (CallFunction|CompleteQuest "S2004")))

(event EventBindNPCActions
  (|CallParentFunction)
  (CallFunction|BindNPCWitnessActions)
  (CallFunction|BindNPCDriverActions))

(event Custom|StartEndConversation
  (if (CallFunction|IsQuestCompleted "S2009")
    (Default|StartNewDialog (Variables|/Game/Game/Blueprints/Tutorial/BP_TutorialBuddy.BP_TutorialBuddy_C|GetAC_TuddyDialogManager (Variables|Tutorial|GetTutorialBuddy)) "S2003")
    (Rendering|SetActorHiddenInGame (Variables|Default|GetDescriptionPanel) true)))

(event Custom|OnTuddyDialogCompleted
  (params (DialogID :type Name))
  (switch name DialogID
    (:S2001
      (Default|Hide (Variables|Tutorial|GetTutorialBuddy))
      (Default|StartDescription (Variables|Default|GetDescriptionPanel))
      (CallFunction|SetQuestList))
    (:S2002
      (for _array_element (Variables|Default|GetSmallRoomMeshes)
        (Actor|DestroyActor _array_element)
        (Utilities|FlowControl|Delay 1.0)
        (Default|Hide (Variables|Tutorial|GetTutorialBuddy))))
    (:S2003
      (Utilities|FlowControl|Delay 0.5)
      (CallFunction|EndGameplay))))

(event EventBindTuddyActions
  (|CallParentFunction)
  (EventDispatchers|BindEventtoEDDialogCompleted (Variables|/Game/Game/Blueprints/Tutorial/BP_TutorialBuddy.BP_TutorialBuddy_C|GetAC_TuddyDialogManager (Variables|Tutorial|GetTutorialBuddy)) (delegate Custom|OnTuddyDialogCompleted)))

(fn ConstructionScript
  (|CallParentFunction))

(fn SetQuestList
  (bind _outrownames (DataTable|GetDataTableRowNames (Variables|Default|GetQuest%20Data%20Table)))
  (for _array_element _outrownames
    (bind _returnvalue (Utilities|GetDataTableRow (Variables|Default|GetQuest%20Data%20Table) _array_element)
      (:then
        (Utilities|Map|Add (LocalVariables|GetQuests) _array_element (.TrackingDescription (Utilities|Struct|BreakF_QuestData _returnvalue))))))
  (Default|SetQuestList (Variables|Default|GetDescriptionPanel) (LocalVariables|GetQuests)))