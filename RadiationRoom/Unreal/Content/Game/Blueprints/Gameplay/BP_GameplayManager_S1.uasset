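; Gameplay manager subclass for scenario S1, which starts with a dialog from the StartTuddy guide.
; When that dialog completes, it hides StartTuddy, opens and locks the big room door, fills the quest list widgets from a data table and sets the first quest.
; A quest progression chain driving NPC conversations, place points, EndTuddy and gameplay end exists but is disconnected from CompleteQuest, so it never runs.
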(event EventBeginPlay
  (|CallParentFunction))

(event EventCompleteQuest
  (params (QuestID :type Name :default "None")))

(event EventStartScenario
  (|CallParentFunction)
  (Utilities|FlowControl|Delay 1.0)
  (Default|StartNewDialog (Variables|/Game/Game/Blueprints/Tutorial/BP_TutorialBuddy.BP_TutorialBuddy_C|GetAC_TuddyDialogManager (Variables|Tuddy|GetStartTuddy)) "S1001"))

(event Custom|OnStartTuddyDialogCompleted
  (params (DialogID :type Name))
  (Utilities|FlowControl|Delay 1.0)
  (Default|Hide (Variables|Tuddy|GetStartTuddy))
  (Default|AutomaticOpenandLockDoor (Variables|Door|GetBigRoomDoor))
  (CallFunction|SetQuestList)
  (for _array_element (Variables|Default|GetQuestListWidget)
    (Rendering|SetActorHiddenInGame _array_element false))
  (CallFunction|SetCurrentQuest "S1001"))

(event EventBindTuddyActions
  (|CallParentFunction)
  (EventDispatchers|BindEventtoEDDialogCompleted (Variables|/Game/Game/Blueprints/Tutorial/BP_TutorialBuddy.BP_TutorialBuddy_C|GetAC_TuddyDialogManager (Variables|Tuddy|GetStartTuddy)) (delegate Custom|OnStartTuddyDialogCompleted)))

(fn ConstructionScript)

(fn SetQuestList
  (bind _outrownames (DataTable|GetDataTableRowNames (Variables|Default|GetQuest%20Data%20Table)))
  (for _array_element _outrownames
    (bind _returnvalue (Utilities|GetDataTableRow (Variables|Default|GetQuest%20Data%20Table) _array_element)
      (:then
        (Utilities|Map|Add (LocalVariables|GetQuests) _array_element (.TrackingDescription (Utilities|Struct|BreakF_QuestData _returnvalue))))))
  (for _array_element_2 (Variables|Default|GetQuestListWidget)
    (Default|SetQuestList _array_element_2 (LocalVariables|GetQuests))))