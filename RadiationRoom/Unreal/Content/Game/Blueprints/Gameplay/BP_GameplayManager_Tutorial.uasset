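; Tutorial gameplay manager that runs the scenario from Tuddy's intro dialog to its farewell, extending a parent manager.
; After the intro, a welcome countdown teleports the player, sets the first quest and starts the first tutorial display.
; Unlocked tasks activate quest elements, completed quests advance displays, and both log events to the database.
; Completing gameplay shows the end Tuddy and goodbye widget, whose post-dialog countdown ends gameplay; cheat keys trigger videos and tasks.
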(event Custom|OnTutorialTaskUnlocked
  (Variables|/Game/Game/Blueprints/Gameplay/BP_GameplayManager.BP_GameplayManager_C|SetStartQuestAllowed (CallFunction|GetMyGameplayManager) true)
  (CallFunction|SendTutorialTaskEventtoDB "NewEnumerator1")
  (Default|ActivateQuestElements (CallFunction|GetCurrentQuestActor)))

(event EventBeginPlay
  (|CallParentFunction)
  (Variables|Default|SetStartQuestAllowed false)
  (Rendering|SetActorHiddenInGame (Variables|Default|GetGoodbyeWidget) true)
  (Default|OnGameInstanceDefaultVarsSetted (Variables|Tutorial|GetTutorialManager)))

(event EventStartScenario
  (|CallParentFunction)
  (Default|Show (Variables|Default|GetStartTuddy)))

(event EventCompleteQuest
  (params (QuestID :type Name :default "None"))
  (|CallParentFunction QuestID)
  (Utilities|FlowControl|Sequence
    (:then_0
      (Default|NextDisplay (Variables|Default|GetTutorialDisplayManager))
      (CallFunction|SendTutorialTaskEventtoDB "NewEnumerator2"))
    (:then_1
      (if (CallFunction|IsGameplayCompleted)
        (Utilities|FlowControl|Delay 1.0)
        (Default|Show (Variables|Default|GetEndTuddy))
        (Rendering|SetActorHiddenInGame (Variables|Default|GetGoodbyeWidget) false)))))

(event Custom|StartVideoKeyPressed
  (Default|CheatKeyStartVideo (Variables|/Game/Game/Blueprints/Tutorial/BP_TutorialDisplay.BP_TutorialDisplay_C|GetExplanation%20Widget%20Actor (Variables|/Game/Game/Blueprints/Tutorial/BP_TutorialDisplayManager.BP_TutorialDisplayManager_C|GetCurrentDisplay (Variables|Default|GetTutorialDisplayManager)))))

(event Custom|OnGoodbyeCountdownCompleted
  (CallFunction|EndGameplay))

(event Custom|StartTaskKeyPressed
  (Default|CheatKeyStartTask (Variables|/Game/Game/Blueprints/Tutorial/BP_TutorialDisplay.BP_TutorialDisplay_C|GetUserTaskWidgetActor (Variables|/Game/Game/Blueprints/Tutorial/BP_TutorialDisplayManager.BP_TutorialDisplayManager_C|GetCurrentDisplay (Variables|Default|GetTutorialDisplayManager)))))

(event Custom|OnStartTuddyDialogCompleted
  (params (DialogID :type Name))
  (bind _welcomewidget (Variables|Default|GetWelcomeWidget))
  (Default|Hide (Variables|Default|GetStartTuddy))
  (Rendering|SetActorHiddenInGame _welcomewidget false)
  (Default|StartCountdown _welcomewidget)
  (EventDispatchers|BindEventtoEDCountdownEnded _welcomewidget (delegate Custom|OnWelcomeCountdownCompleted)))

(event Custom|OnEndTuddyDialogCompleted
  (params (DialogID :type Name))
  (bind _goodbyewidget (Variables|Default|GetGoodbyeWidget))
  (Default|Hide (Variables|Default|GetEndTuddy))
  (Rendering|SetActorHiddenInGame _goodbyewidget false)
  (Default|StartCountdown _goodbyewidget)
  (EventDispatchers|BindEventtoEDCountdownEnded _goodbyewidget (delegate Custom|OnGoodbyeCountdownCompleted)))

(event Custom|OnWelcomeCountdownCompleted
  (Transformation|SetActorLocation (CallFunction|GetMyPlayer) (Transformation|GetActorLocation (Variables|Default|GetInitialTeleportPoint)) false true)
  (bind _keys (Utilities|Map|Keys (Variables|Default|GetQuestActorList)))
  (CallFunction|SetCurrentQuest (Utilities|Array|Get(acopy) _keys))
  (Default|StartFirstDisplay (Variables|Default|GetTutorialDisplayManager)))

(event EventBindTuddyActions
  (|CallParentFunction)
  (EventDispatchers|BindEventtoEDDialogCompleted (Variables|/Game/Game/Blueprints/Tutorial/BP_TutorialBuddy.BP_TutorialBuddy_C|GetAC_DialogManager_Tuddy (Variables|Default|GetStartTuddy)) (delegate Custom|OnStartTuddyDialogCompleted))
  (EventDispatchers|BindEventtoEDDialogCompleted (Variables|/Game/Game/Blueprints/Tutorial/BP_TutorialBuddy.BP_TutorialBuddy_C|GetAC_DialogManager_Tuddy (Variables|Default|GetEndTuddy)) (delegate Custom|OnEndTuddyDialogCompleted)))

(event Custom|SendTutorialTaskEventToDB
  (params (Event%20State :type E_TutorialTaskEventType%20Enum :default "NewEnumerator0"))
  (bind _database_manager (CallFunction|GetMyDataBase))
  (bind _data (Default|GetDataBaseMainInfoEvent (CallFunction|GetMyGameInstance)))
  (Utilities|IsValid _database_manager
    (:Is%20Valid
      (Default|SendTutorialTaskEvent _database_manager (Utilities|Struct|MakeF_TutorialTaskEvent 0 (.user_id (Utilities|Struct|BreakF_MainInfoEvent _data)) (.experiment_id (Utilities|Struct|BreakF_MainInfoEvent _data)) (.scenario_type (Utilities|Struct|BreakF_MainInfoEvent _data)) (Variables|Tutorial|GetCurrent%20Tutorial%20Item%20Id) Event%20State (Math|DateTime|Now))))))

(fn ConstructionScript
  (|CallParentFunction))