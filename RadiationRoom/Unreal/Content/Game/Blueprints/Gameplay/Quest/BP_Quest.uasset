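; Base quest Blueprint that tracks started and completed state, with empty Init and ActivateQuestElements events as hooks.
; Starting or completing a quest sends a timestamped gameplay event with user, experiment and scenario info to the database manager, if valid.
; Completion also notifies the gameplay manager, which is fetched, like the game instance, through the quest's outer object.
; CanStartQuest requires both the Started flag and the manager's StartQuestAllowed.
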(event Custom|StartQuest
  (Variables|Default|SetStarted true)
  (CallFunction|SendQuesttoDatabase (Variables|Default|GetId) "NewEnumerator1"))

(event Custom|CompleteQuest
  (Variables|Default|SetStarted false)
  (Variables|Default|SetCompleted true)
  (CallFunction|SendQuesttoDatabase (Variables|Default|GetId) "NewEnumerator3")
  (Default|CompleteQuest (CallFunction|GetGameplayManager) (Variables|Default|GetId)))

(event Custom|ActivateQuestElements)

(event Custom|Init)

(fn SendQuesttoDatabase
  (params (Quest%20ID :type Name) (Step%20State :type E_QuestState%20Enum :default "NewEnumerator0"))
  (bind _gameinstance (CallFunction|GetGameInstance))
  (bind _database_manager (Variables|/Game/Game/Blueprints/RR_GameInstance.RR_GameInstance_C|GetDatabase%20Manager _gameinstance))
  (bind _data (Default|GetDataBaseMainInfoEvent (CallFunction|GetGameInstance)))
  (Utilities|IsValid _database_manager
    (:Is%20Valid
      (Default|SendGameplayEventtoDB _database_manager (Utilities|Struct|MakeF_GameplayEvent 0 (.user_id (Utilities|Struct|BreakF_MainInfoEvent _data)) (.experiment_id (Utilities|Struct|BreakF_MainInfoEvent _data)) (.scenario_type (Utilities|Struct|BreakF_MainInfoEvent _data)) Quest%20ID Step%20State (Math|DateTime|Now))))))

(fn GetGameplayManager
  (return (CallFunction|GetMyGameplayManager (Utilities|GetOuterObject self))))

(fn GetGameInstance
  (return (CallFunction|GetMyGameInstance (Utilities|GetOuterObject self))))

(fn CanStartQuest
  (return (and (Variables|Default|GetStarted) (Variables|/Game/Game/Blueprints/Gameplay/BP_GameplayManager.BP_GameplayManager_C|GetStartQuestAllowed (CallFunction|GetGameplayManager)))))