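; Quest Blueprint for T2 SAB, which tasks the player with measuring radiation on both an item and an NPC using the SABG100 dosimeter.
; On start, it binds to the item and NPC measurement events of every SABG100 dosimeter in the level.
; Readings count only once quest elements are activated and the quest can start.
; Both flags feed a shared check that completes the quest, in either order.
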(event Custom|OnSABG100ItemRadiationMeasured
  (params (Actor :type BP%20Interact%20Item%20Parent%20Object%20Reference))
  (if (and (CallFunction|CanStartQuest) (Variables|Default|GetCanUseSABG100))
    (Variables|Default|SetItem%20Radiation%20Measured true)
    (if (and (Variables|Default|GetItem%20Radiation%20Measured) (Variables|Default|GetNPCRadiation%20Measured))
      (CallFunction|CompleteQuest))))

(event Custom|ONSABG100NPCRadiationMeasured
  (params (Actor :type BP%20NPC%20Object%20Reference))
  (if (and (CallFunction|CanStartQuest) (Variables|Default|GetCanUseSABG100))
    (Variables|Default|SetNPCRadiation%20Measured true)
    (if (and (Variables|Default|GetItem%20Radiation%20Measured) (Variables|Default|GetNPCRadiation%20Measured))
      (CallFunction|CompleteQuest))))

(event EventInit
  (params (GameplayManager :type BP%20Gameplay%20Manager%20Object%20Reference))
  (|CallParentFunction GameplayManager)
  (Variables|Default|SetCanUseSABG100 false))

(event EventStartQuest
  (|CallParentFunction)
  (bind _outactors (Actor|GetAllActorsOfClass (Utilities|GetOuterObject self) "/Game/Game/Blueprints/Actors/Dosimeters/BP_Dosimeter_SABG100.BP_Dosimeter_SABG100_C"))
  (for _array_element _outactors
    (EventDispatchers|AssignEDItemRadiationMeasured _array_element (delegate Custom|OnSABG100ItemRadiationMeasured))
    (EventDispatchers|AssignEDNPCRadiationMeasured _array_element (delegate Custom|ONSABG100NPCRadiationMeasured))))

(event EventActivateQuestElements
  (Variables|Default|SetCanUseSABG100 true))