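; Tier 2 RBQ quest that completes once the player has spawned at least two traffic cones and one SABG100 from the RBQ van.
; On init it finds the BP_RBQVan in the world through its outer object and binds to the van's item-spawned event.
; Each spawn, if the quest can start, increments a counter by item type and then checks both totals to complete the quest.
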(event Custom|OnRBQItemSpawned
  (params (Actor :type BP%20Item%20Initial%20State%20Object%20Reference))
  (if (CallFunction|CanStartQuest)
    (Utilities|FlowControl|Sequence
      (:then_0
        (switch Utilities|FlowControl|Switch|SwitchonE_ItemType (Variables|/Game/Game/Blueprints/Actors/Items/BP_ItemInitialState.BP_ItemInitialState_C|GetItemType Actor)
          (:NewEnumerator0
            (bind _result (Math|Integer|IncrementInt (Variables|Default|GetNumOfTrafficConesSpawned))
              (:%20%20
                (Variables|Default|SetNumOfTrafficConesSpawned _result))))
          (:NewEnumerator1
            (bind _result_2 (Math|Integer|IncrementInt (Variables|Default|GetNumOfSABG100Spawned))
              (:%20%20
                (Variables|Default|SetNumOfSABG100Spawned _result_2))))))
      (:then_1
        (if (and (>= (Variables|Default|GetNumOfTrafficConesSpawned) 2) (>= (Variables|Default|GetNumOfSABG100Spawned) 1))
          (CallFunction|CompleteQuest))))))

(event EventInit
  (params (GameplayManager :type BP%20Gameplay%20Manager%20Object%20Reference))
  (|CallParentFunction GameplayManager)
  (bind _returnvalue (Actor|GetActorOfClass (Utilities|GetOuterObject self) "/Game/Game/Blueprints/Actors/BP_RBQVan.BP_RBQVan_C"))
  (bind _output_get (Variables|Default|SetRBQVan _returnvalue))
  (EventDispatchers|BindEventtoEDItemSpawned _output_get (delegate Custom|OnRBQItemSpawned)))