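; Quest logic for the T2 scenario that completes when the player brings a held EPD dosimeter to the radiation emission point.
; On init it binds to the T2 gameplay manager's radiation emission sphere trigger overlap.
; The overlap only counts once quest activation enables EPD use, the dosimeter is grabbed and the quest can start, then it completes after a one-second delay.
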(event Custom|OnEPDOverlapped
  (params (OverlappedActor :type Actor%20Object%20Reference) (OtherActor :type Actor%20Object%20Reference))
  (bind _asbp_dosimeter_epd (Utilities|Casting|CastToBP_Dosimeter_EPD OtherActor))
  (if (Math|Boolean|ANDBoolean (Variables|/Game/Game/Blueprints/Actors/Items/BP_PickableItem.BP_PickableItem_C|GetGrabbed _asbp_dosimeter_epd) (CallFunction|CanStartQuest) (Variables|Default|GetCanUseEPD))
    (Utilities|FlowControl|Delay (Utilities|GetOuterObject self) 1.0)
    (CallFunction|CompleteQuest)))

(event EventInit
  (params (GameplayManager :type BP%20Gameplay%20Manager%20Object%20Reference))
  (|CallParentFunction GameplayManager)
  (Variables|Default|SetCanUseEPD false)
  (bind _asbp_gameplay_manager_t2 (Utilities|Casting|CastToBP_GameplayManager_T2 (Variables|Default|GetGameplay%20Manager)))
  (Collision|BindEventtoOnActorBeginOverlap (Variables|/Game/Game/Blueprints/Gameplay/BP_GameplayManager_T2.BP_GameplayManager_T2_C|GetRadiationEmissionPointSphereTrigger _asbp_gameplay_manager_t2) (delegate Custom|OnEPDOverlapped)))

(event EventActivateQuestElements
  (Variables|Default|SetCanUseEPD true))