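; BP_Quest_T2_WAL is a tier-T2 quest built around the walkie-talkie's initial report.
; On init it finds the BP_WalkieTalkie in the level, disables its dialog box and binds to its initial-report-completed event.
; Activating the quest elements re-enables the dialog box.
; When the report completes, the quest completes if it is able to start.
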(event Custom|OnWalkieInitialReportCompleted
  (if (CallFunction|CanStartQuest)
    (CallFunction|CompleteQuest)))

(event EventInit
  (params (GameplayManager :type BP%20Gameplay%20Manager%20Object%20Reference))
  (|CallParentFunction GameplayManager)
  (bind _returnvalue (Actor|GetActorOfClass (Utilities|GetOuterObject self) "/Game/Game/Blueprints/WalkieTalkie/BP_WalkieTalkie.BP_WalkieTalkie_C"))
  (bind _output_get (Variables|Default|SetWalkie-%20Talkie _returnvalue))
  (Variables|/Game/Game/Blueprints/WalkieTalkie/BP_WalkieTalkie.BP_WalkieTalkie_C|SetCanShowDialogBox _output_get false)
  (EventDispatchers|BindEventtoEDInitialReportCompleted _output_get (delegate Custom|OnWalkieInitialReportCompleted)))

(event EventActivateQuestElements
  (Variables|/Game/Game/Blueprints/WalkieTalkie/BP_WalkieTalkie.BP_WalkieTalkie_C|SetCanShowDialogBox (Variables|Default|GetWalkie-%20Talkie) true))