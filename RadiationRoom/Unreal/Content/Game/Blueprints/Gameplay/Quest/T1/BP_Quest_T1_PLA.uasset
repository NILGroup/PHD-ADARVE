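; BP_Quest_T1_PLA is a T1 quest that completes once every place point manager has all its points used.
; On Init it takes the managers from BP_GameplayManager_T1, disables their point activation and binds to their all-points-with-items event.
; Activating the quest elements re-enables the points.
; Each manager's completion event rechecks CanStartQuest and every manager's AllPointsUsed before completing the quest.
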(event Custom|OnPlacePointManagerCompleted
  (if (and (CallFunction|CanStartQuest) (CallFunction|AllPlacePointManagersCompleted))
    (CallFunction|CompleteQuest)))

(event EventInit
  (params (GameplayManager :type BP%20Gameplay%20Manager%20Object%20Reference))
  (|CallParentFunction GameplayManager)
  (bind _asbp_gameplay_manager_t1 (Utilities|Casting|CastToBP_GameplayManager_T1 (Variables|Default|GetGameplay%20Manager)))
  (bind _output_get (Variables|Default|SetPlacePointManagers (Variables|/Game/Game/Blueprints/Gameplay/BP_GameplayManager_T1.BP_GameplayManager_T1_C|GetPlacePointManagers _asbp_gameplay_manager_t1)))
  (for _array_element _output_get
    (Variables|/Game/Game/Blueprints/Actors/Items/PlacePoints/BP_PlacePointManager.BP_PlacePointManager_C|SetCanActivatePoints _array_element false)
    (EventDispatchers|BindEventtoEDAllPlacePointswithItems _array_element (delegate Custom|OnPlacePointManagerCompleted))))

(event EventActivateQuestElements
  (|CallParentFunction)
  (for _array_element (Variables|Default|GetPlacePointManagers)
    (Variables|/Game/Game/Blueprints/Actors/Items/PlacePoints/BP_PlacePointManager.BP_PlacePointManager_C|SetCanActivatePoints _array_element true)))

(fn AllPlacePointManagersCompleted
  (bind _array_element (Utilities|Array|ForEachLoopwithBreak (Variables|Default|GetPlacePointManagers) :!label _label)
    (:LoopBody
      (if (not (Variables|/Game/Game/Blueprints/Actors/Items/PlacePoints/BP_PlacePointManager.BP_PlacePointManager_C|GetAllPointsUsed _array_element))
        (LocalVariables|SetPlace%20Completed false)
        (goto _label Break)))
    (:Completed
      (return (LocalVariables|GetPlace%20Completed)))))