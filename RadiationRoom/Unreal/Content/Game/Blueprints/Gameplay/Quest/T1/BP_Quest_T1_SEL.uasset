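; Tutorial quest object that completes once enough distinct pickable items have been selected.
; Init gathers every BP_PickableItem in the world, using the outer object as context, and binds each one's detection-started event to the selection handler.
; While CanStartQuest passes, the handler records each new actor in SelectedActors and calls CompleteQuest when the added index reaches MaxSelectedActors minus one.
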(event Custom|OnTutorialItemSelected
  (params (Actor :type BP%20Interact%20Item%20Parent%20Object%20Reference))
  (bind _selectedactors (Variables|Default|GetSelectedActors))
  (if (CallFunction|CanStartQuest)
    (if (not (Utilities|Array|ContainsItem _selectedactors Actor))
      (bind _returnvalue (Utilities|Array|Add _selectedactors Actor))
      (if (== _returnvalue (- (Variables|Default|GetMaxSelectedActors) 1))
        (CallFunction|CompleteQuest)))))

(event EventInit
  (bind _outactors (Actor|GetAllActorsOfClass (Utilities|GetOuterObject self) "/Game/Game/Blueprints/Actors/Items/BP_PickableItem.BP_PickableItem_C"))
  (bind _output_get (Variables|Default|SetSelectableItemsList _outactors))
  (for _array_element _output_get
    (EventDispatchers|BindEventtoEDDetectionStarted _array_element (delegate Custom|OnTutorialItemSelected))))