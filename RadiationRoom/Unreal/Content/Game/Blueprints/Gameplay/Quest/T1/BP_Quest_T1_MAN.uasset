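; Tutorial quest that completes once enough different pickable items have been manipulated.
; On init it gathers every BP_PickableItem actor in the world and binds to each one's detection-started event.
; While the quest can start, each newly detected item is added once to a tracked list, and reaching the maximum count completes the quest.
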(event Custom|OnTutorialItemManipulated
  (params (Actor :type BP%20Interact%20Item%20Parent%20Object%20Reference))
  (bind _manipuledactors (Variables|Default|GetManipuledActors))
  (if (CallFunction|CanStartQuest)
    (if (not (Utilities|Array|ContainsItem _manipuledactors Actor))
      (bind _returnvalue (Utilities|Array|Add _manipuledactors Actor))
      (if (== _returnvalue (- (Variables|Default|GetMaxManipuledActors) 1))
        (CallFunction|CompleteQuest)))))

(event EventInit
  (params (GameplayManager :type BP%20Gameplay%20Manager%20Object%20Reference))
  (|CallParentFunction GameplayManager)
  (bind _outactors (Actor|GetAllActorsOfClass (Utilities|GetOuterObject self) "/Game/Game/Blueprints/Actors/Items/BP_PickableItem.BP_PickableItem_C"))
  (bind _output_get (Variables|Default|SetManipulableItemsList _outactors))
  (for _array_element _output_get
    (EventDispatchers|BindEventtoEDDetectionStarted _array_element (delegate Custom|OnTutorialItemManipulated))))