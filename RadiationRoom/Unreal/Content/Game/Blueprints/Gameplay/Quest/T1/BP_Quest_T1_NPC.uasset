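; BP_Quest_T1_NPC is a T1 quest that completes when the player finishes a conversation with an NPC.
; On init it takes the NPC from the T1 gameplay manager and binds to its conversation-finished event.
; Activating the quest lets the NPC talk and rechecks player overlap.
; When a conversation ends and the quest can start, it completes and advances the NPC to the next conversation.
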(event Custom|OnNPCConversationFinished
  (params (ConversationNumber :type Integer))
  (if (CallFunction|CanStartQuest)
    (CallFunction|CompleteQuest)
    (Default|NextConversation (Variables|Default|GetNPC))))

(event EventActivateQuestElements
  (bind _npc (Variables|Default|GetNPC))
  (Variables|/Game/Game/Blueprints/Characters/BP_NPC_Talkable.BP_NPC_Talkable_C|SetCanTalk _npc true)
  (Default|PlayerIsAlreadyOverlapping _npc))

(event EventInit
  (params (GameplayManager :type BP%20Gameplay%20Manager%20Object%20Reference))
  (|CallParentFunction GameplayManager)
  (bind _asbp_gameplay_manager_t1 (Utilities|Casting|CastToBP_GameplayManager_T1 (Variables|Default|GetGameplay%20Manager)))
  (bind _output_get (Variables|Default|SetNPC (Variables|/Game/Game/Blueprints/Gameplay/BP_GameplayManager_T1.BP_GameplayManager_T1_C|GetNPC _asbp_gameplay_manager_t1)))
  (EventDispatchers|BindEventtoEDConversationFinished _output_get (delegate Custom|OnNPCConversationFinished)))