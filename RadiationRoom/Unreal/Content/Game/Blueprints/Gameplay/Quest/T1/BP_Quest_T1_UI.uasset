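; BP_Quest_T1_UI is a T1 quest that completes when all buttons on an interactive panel have been clicked.
; On Init it gets the panel actor from the T1 gameplay manager, hides it and binds to its all-buttons-clicked dispatcher.
; Activating the quest elements reveals the panel, and the dispatcher's callback completes the quest.
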(event Custom|OnAllButtonsClicked
  (CallFunction|CompleteQuest))

(event EventInit
  (bind _asbp_gameplay_manager_t1 (Utilities|Casting|CastToBP_GameplayManager_T1 (CallFunction|GetGameplayManager)))
  (Variables|Default|SetInteractivePanel (Variables|/Game/Game/Blueprints/Gameplay/BP_GameplayManager_T1.BP_GameplayManager_T1_C|GetInteractivePanelActor _asbp_gameplay_manager_t1))
  (Rendering|SetActorHiddenInGame (Variables|Default|GetInteractivePanel) true)
  (EventDispatchers|BindEventtoEDAllButtonsClicked (Variables|Default|GetInteractivePanel) (delegate Custom|OnAllButtonsClicked)))

(event EventActivateQuestElements
  (Rendering|SetActorHiddenInGame (Variables|Default|GetInteractivePanel) false))