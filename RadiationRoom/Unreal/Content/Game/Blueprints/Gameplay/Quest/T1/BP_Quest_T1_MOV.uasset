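; Tier 1 movement quest Blueprint that completes after the player teleports five times.
; On start, it binds to the teleported event dispatcher of the player obtained from the quest's outer object.
; Each teleport increments a counter while the CanStartQuest check passes, and the quest completes when the count reaches five.
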(event Custom|OnPlayerTeleported
  (if (CallFunction|CanStartQuest)
    (bind _output_get (Variables|Default|SetTimesTeleported (+ (Variables|Default|GetTimesTeleported) 1)))
    (if (== _output_get 5)
      (CallFunction|CompleteQuest))))

(event EventStartQuest
  (|CallParentFunction)
  (EventDispatchers|BindEventtoEDTeleported (CallFunction|GetMyPlayer (Utilities|GetOuterObject self)) (delegate Custom|OnPlayerTeleported)))

(event EventInit
  (params (GameplayManager :type BP%20Gameplay%20Manager%20Object%20Reference))
  (|CallParentFunction GameplayManager))