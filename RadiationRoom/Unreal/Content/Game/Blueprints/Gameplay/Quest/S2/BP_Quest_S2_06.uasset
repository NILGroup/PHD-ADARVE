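; Quest S2_06, a scenario 2 quest that completes when an item, apparently a traffic cone, is placed at a place point.
; On Init it finds the BP_PlacePointManager and binds to its one-item-placed event.
; The first placement completes the quest and turns on collision for the S2 gameplay manager's TrafficWall.
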(event Custom|OnOneTrafficConeHasBeenPlaced
  (params (Item :type BP%20Pickable%20Item%20Object%20Reference) (PlacePoint :type BP%20Place%20Point%20Object%20Reference))
  (if (not (Variables|Default|GetCompleted))
    (CallFunction|CompleteQuest)
    (bind _asbp_gameplay_manager_s2 (Utilities|Casting|CastToBP_GameplayManager_S2 (Variables|Default|GetGameplay%20Manager)))
    (Collision|SetActorEnableCollision (Variables|/Game/Game/Blueprints/Gameplay/BP_GameplayManager_S2.BP_GameplayManager_S2_C|GetTrafficWall _asbp_gameplay_manager_s2) true)))

(event EventInit
  (params (GameplayManager :type BP%20Gameplay%20Manager%20Object%20Reference))
  (|CallParentFunction GameplayManager)
  (bind _returnvalue (Actor|GetActorOfClass (Utilities|GetOuterObject self) "/Game/Game/Blueprints/Actors/Items/PlacePoints/BP_PlacePointManager.BP_PlacePointManager_C"))
  (EventDispatchers|AssignEDOneItemHasBeenPlaced _returnvalue (delegate Custom|OnOneTrafficConeHasBeenPlaced)))