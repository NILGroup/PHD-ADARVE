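; Quest Blueprint for S2 quest 01, completed when any tracked walkie-talkie makes its initial report.
; Each new walkie-talkie has both report flags reset, binds its initial-report event to the quest and joins a tracked list.
; If the quest is still open when a report arrives, it marks the initial report done on every listed walkie-talkie and completes the quest.
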(event Custom|NewWalkieTalkie
  (params (Walkie%20Talkie :type BP%20Walkie%20Talkie%20Object%20Reference))
  (Default|SetInitialReportCompleted Walkie%20Talkie false)
  (Default|SetFinalReportCompleted Walkie%20Talkie false)
  (CallFunction|BindWalkieTalkieEvents Walkie%20Talkie)
  (Utilities|Array|Add (Variables|Default|GetWalkieTalkieList) Walkie%20Talkie))

(event Custom|BindWalkieTalkieEvents
  (params (WalkieTalkie :type BP%20Walkie%20Talkie%20Object%20Reference))
  (EventDispatchers|BindEventtoEDInitialReportCompleted WalkieTalkie (delegate Custom|OnWalkieInitialReportCompleted)))

(event Custom|OnWalkieInitialReportCompleted
  (if (not (Variables|Default|GetCompleted))
    (for _array_element (Variables|Default|GetWalkieTalkieList)
      (Default|SetInitialReportCompleted _array_element true))
    (CallFunction|CompleteQuest)))

(event EventInit
  (params (GameplayManager :type BP%20Gameplay%20Manager%20Object%20Reference))
  (|CallParentFunction GameplayManager))