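; BP_Quest_S2_08 is a scenario 2 quest that completes when the player measures radiation on the radioactive item with an SABG100 device.
; It binds to the item-measured event of each new SABG100 and keeps the devices in a list.
; A measurement completes the quest if it is not already done and the measured actor matches the RadiactiveItem held by the S2 gameplay manager.
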(event Custom|New%20SABG100
  (params (SABG100 :type BP%20Dosimeter%20SABG100%20Object%20Reference))
  (EventDispatchers|BindEventtoEDItemRadiationMeasured SABG100 (delegate Custom|OnSABG100ItemRadiationMeasured))
  (Utilities|Array|Add (Variables|Default|GetSABG100List) SABG100))

(event Custom|OnSABG100ItemRadiationMeasured
  (params (Actor :type BP%20Interact%20Item%20Parent%20Object%20Reference))
  (if (not (Variables|Default|GetCompleted))
    (bind _asbp_gameplay_manager_s2 (Utilities|Casting|CastToBP_GameplayManager_S2 (Variables|Default|GetGameplay%20Manager)))
    (if (== (Variables|/Game/Game/Blueprints/Gameplay/BP_GameplayManager_S2.BP_GameplayManager_S2_C|GetRadiactiveItem _asbp_gameplay_manager_s2) Actor)
      (CallFunction|CompleteQuest))))

(event EventInit
  (params (GameplayManager :type BP%20Gameplay%20Manager%20Object%20Reference))
  (|CallParentFunction GameplayManager))