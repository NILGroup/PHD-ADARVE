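; BP_Quest_S1_01 is a Season or Stage 1 quest that completes when the player enters the big room.
; On Init it gets the S1 gameplay manager and binds to its BigRoomTrigger overlap event.
; When an actor overlaps that trigger, it completes the quest if it can start and the actor is the local player.
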(event Custom|OnActorEnterInBigRoom
  (params (OverlappedActor :type Actor%20Object%20Reference) (OtherActor :type Actor%20Object%20Reference))
  (if (and (CallFunction|CanStartQuest) (== OtherActor (CallFunction|GetMyPlayer (Utilities|GetOuterObject self))))
    (CallFunction|CompleteQuest)))

(event EventInit
  (bind _asbp_gameplay_manager_s1 (Utilities|Casting|CastToBP_GameplayManager_S1 (CallFunction|GetGameplayManager)))
  (Collision|BindEventtoOnActorBeginOverlap (Variables|/Game/Game/Blueprints/Gameplay/BP_GameplayManager_S1.BP_GameplayManager_S1_C|GetBigRoomTrigger _asbp_gameplay_manager_s1) (delegate Custom|OnActorEnterInBigRoom)))