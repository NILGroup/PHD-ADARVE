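; Quest blueprint for the third S1 quest, a tidy-up phase in which items fill place points.
; Init binds to each S1 gameplay manager place point manager's all-points-filled event.
; StartQuest enables those points and shows their info widgets.
; Each completion event checks CanStartQuest and whether all managers' points are used, then completes the quest and advances the NPC to its next conversation.
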(event Custom|OnPlacePointManagerCompleted
  (if (CallFunction|CanStartQuest)
    (bind _completed (CallFunction|IsTidyUpPhaseCompleted?))
    (if _completed
      (CallFunction|CompleteQuest))))

(event EventInit
  (params (GameplayManager :type BP%20Gameplay%20Manager%20Object%20Reference))
  (|CallParentFunction GameplayManager)
  (bind _asbp_gameplay_manager_s1 (Utilities|Casting|CastToBP_GameplayManager_S1 (Variables|Default|GetGameplay%20Manager)))
  (for _array_element (Variables|/Game/Game/Blueprints/Gameplay/BP_GameplayManager_S1.BP_GameplayManager_S1_C|GetPlacePointManagers _asbp_gameplay_manager_s1)
    (EventDispatchers|BindEventtoEDAllPlacePointswithItems _array_element (delegate Custom|OnPlacePointManagerCompleted))))

(event EventCompleteQuest
  (|CallParentFunction)
  (bind _asbp_gameplay_manager_s1 (Utilities|Casting|CastToBP_GameplayManager_S1 (Variables|Default|GetGameplay%20Manager)))
  (Default|NextConversation (Variables|/Game/Game/Blueprints/Gameplay/BP_GameplayManager_S1.BP_GameplayManager_S1_C|GetNPC _asbp_gameplay_manager_s1)))

(event EventStartQuest
  (|CallParentFunction)
  (bind _asbp_gameplay_manager_s1 (Utilities|Casting|CastToBP_GameplayManager_S1 (Variables|Default|GetGameplay%20Manager)))
  (for _array_element (Variables|/Game/Game/Blueprints/Gameplay/BP_GameplayManager_S1.BP_GameplayManager_S1_C|GetPlacePointManagers _asbp_gameplay_manager_s1)
    (Variables|/Game/Game/Blueprints/Actors/Items/PlacePoints/BP_PlacePointManager.BP_PlacePointManager_C|SetCanActivatePoints _array_element true)
    (Default|ShowInfoWidget _array_element)))

(fn IsTidyUpPhaseCompleted?
  (bind _array_element (Utilities|Array|ForEachLoopwithBreak (Variables|Default|GetPlacePointManagers) :!label _label)
    (:LoopBody
      (if (not (Variables|/Game/Game/Blueprints/Actors/Items/PlacePoints/BP_PlacePointManager.BP_PlacePointManager_C|GetAllPointsUsed _array_element))
        (LocalVariables|SetPlacePointsCompleted false)
        (goto _label Break)))
    (:Completed
      (return (LocalVariables|GetPlacePointsCompleted)))))