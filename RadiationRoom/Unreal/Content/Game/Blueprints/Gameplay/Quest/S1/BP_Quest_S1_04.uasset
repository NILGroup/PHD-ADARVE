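; BP_Quest_S1_04 is a stage 1 quest that completes through an NPC conversation.
; On init it casts the gameplay manager to the S1 manager and binds to the NPC's conversation-finished event.
; When a conversation ends and the quest can start, it completes itself, waits briefly, then shows the manager's EndTuddy.
; The conversation number is not checked, and the delay uses the outer object as world context.
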(event Custom|OnNPCConversationFinished
  (params (ConversationNumber :type Integer))
  (if (CallFunction|CanStartQuest)
    (CallFunction|CompleteQuest)
    (Utilities|FlowControl|Delay (Utilities|GetOuterObject self) 1.5)
    (bind _asbp_gameplay_manager_s1 (Utilities|Casting|CastToBP_GameplayManager_S1 (Variables|Default|GetGameplay%20Manager)))
    (Default|Show (Variables|/Game/Game/Blueprints/Gameplay/BP_GameplayManager_S1.BP_GameplayManager_S1_C|GetEndTuddy _asbp_gameplay_manager_s1))))

(event EventInit
  (params (GameplayManager :type BP%20Gameplay%20Manager%20Object%20Reference))
  (|CallParentFunction GameplayManager)
  (bind _asbp_gameplay_manager_s1 (Utilities|Casting|CastToBP_GameplayManager_S1 (Variables|Default|GetGameplay%20Manager)))
  (EventDispatchers|BindEventtoEDConversationFinished (Variables|/Game/Game/Blueprints/Gameplay/BP_GameplayManager_S1.BP_GameplayManager_S1_C|GetNPC _asbp_gameplay_manager_s1) (delegate Custom|OnNPCConversationFinished)))