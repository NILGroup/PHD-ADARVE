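; Actor component that reveals text one character at a time in a given text widget for a typewriter effect.
; StartTypewriting stores the text, timings and widget, then UpdateText re-calls itself through Delay, growing the displayed substring by one character each pass.
; IsLetter selects the longer-or-shorter punctuation delay after periods, commas, question and exclamation marks.
; When the full string is shown, it calls the TextFullDisplayed event dispatcher.
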(event Custom|StartTypewriting
  (params (Text :type Text) (TimePerChar :type Float%20%28double-precision%29) (TimePerPunctuation :type Float%20%28double-precision%29) (Text%20Widget :type Text%20Block%20Object%20Reference))
  (Utilities|FlowControl|Sequence
    (:then_0
      (Variables|Default|SetFull%20Text (Utilities|String|ToString(Text) Text))
      (Variables|Default|SetCurrent%20Displayed%20Text "")
      (Variables|Default|SetTime%20Per%20Char TimePerChar)
      (Variables|Default|SetTime%20Per%20Punctuation TimePerPunctuation)
      (Variables|Default|SetText%20Widget Text%20Widget))
    (:then_1
      (CallFunction|UpdateText))))

(event Custom|UpdateText
  (Utilities|FlowControl|Sequence
    (:then_0
      (bind _output_get (Variables|Default|SetCurrent%20Displayed%20Text (Utilities|String|GetSubstring (Variables|Default|GetFull%20Text) 0 (+ (Utilities|String|Len (Variables|Default|GetCurrent%20Displayed%20Text)) 1))))
      (Rendering|Components|TextRender|SetText (Variables|Default|GetText%20Widget) (Utilities|Text|ToText(String) _output_get)))
    (:then_1
      (if (Utilities|Enum|Equal(Enum) (Variables|Default|GetFull%20Text) (Variables|Default|GetCurrent%20Displayed%20Text))
        (Default|CallEDTextFullDisplayed)
        (else
          (if (CallFunction|IsLetter?)
            (Utilities|FlowControl|Delay (Variables|Default|GetTime%20Per%20Char))
            (else
              (Utilities|FlowControl|Delay (Variables|Default|GetTime%20Per%20Punctuation))))
          (CallFunction|UpdateText))))))

(event EventBeginPlay)

(event EventTick
  (params (DeltaSeconds :type Float%20%28single-precision%29)))

(fn IsLetter?
  (bind _current_displayed_text (Variables|Default|GetCurrent%20Displayed%20Text))
  (bind _returnvalue (Utilities|String|Len _current_displayed_text))
  (bind _returnvalue_2 (- _returnvalue 1))
  (bind _returnvalue_3 (Utilities|String|GetSubstring _current_displayed_text _returnvalue_2))
  (return (not (Math|Boolean|ORBoolean (Utilities|Enum|Equal(Enum) _returnvalue_3 ".") (Utilities|Enum|Equal(Enum) _returnvalue_3 ",") (Utilities|Enum|Equal(Enum) _returnvalue_3 "?") (Utilities|Enum|Equal(Enum) _returnvalue_3 "!")))))