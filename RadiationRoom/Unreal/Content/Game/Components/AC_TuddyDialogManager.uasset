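; Actor component that runs the tutorial buddy's dialog, showing lines in its speech bubble with matching voice audio.
; StartNewDialog loads lines and audio by ID from a data table, then each line feeds the bubble widget's typewriter text and the buddy's audio component.
; Typewriter completion, not audio length, advances lines after a short delay until the dialog ends, with dispatchers announcing start, stop and completion.
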(event Custom|OnTypewriterCompleted
  (if (Variables|Default|GetIsTalking?)
    (Utilities|FlowControl|Delay 1.5)
    (CallFunction|NextDialog)))

(event Custom|ProcessDialog
  (bind _owner (Variables|Default|GetOwner))
  (bind _dialogaudio (Variables|/Game/Game/Blueprints/Tutorial/BP_TutorialBuddy.BP_TutorialBuddy_C|GetDialogAudio _owner))
  (Default|SetDialogText (Variables|Default|GetWidget) (Utilities|Array|Get(acopy) (Variables|Default|GetCurrentDialogLines) (Variables|Default|GetCurrentDialogIndex)) (Variables|Default|GetTypewriterComponent))
  (Audio|Components|Audio|SetSound _dialogaudio (Utilities|Array|Get(acopy) (Variables|Default|GetCurrentDialogAudios) (Variables|Default|GetCurrentDialogIndex)))
  (Audio|Components|Audio|Play _dialogaudio 0.0))

(event Custom|NextDialog
  (bind _there_are_more_dialogs (CallFunction|MoreDialogLines?))
  (if _there_are_more_dialogs
    (Variables|Default|SetCurrentDialogIndex (+ (Variables|Default|GetCurrentDialogIndex) 1))
    (CallFunction|ProcessDialog)
    (else
      (CallFunction|EndDialog))))

(event Custom|StopDialog
  (Default|HideDialogBubble (Variables|Default|GetOwner))
  (Variables|Default|SetIsTalking? false)
  (Default|CallEDDialogStopped))

(event Custom|EndDialog
  (CallFunction|ResetDialogValues)
  (Default|HideDialogBubble (Variables|Default|GetOwner))
  (Variables|Default|SetIsTalking? false)
  (Default|CallEDDialogCompleted (Variables|Default|GetCurrentDialogID))
  (Variables|Default|SetCurrentDialogID "None"))

(event Custom|ResetDialogValues
  (Utilities|Array|Clear (Variables|Default|GetCurrentDialogLines))
  (Variables|Default|SetCurrentDialogIndex 0))

(event Custom|Init
  (Utilities|FlowControl|Sequence
    (:then_0
      (bind _asbp_tutorial_buddy (Utilities|Casting|CastToBP_TutorialBuddy (Components|GetOwner)))
      (Variables|Default|SetOwner _asbp_tutorial_buddy))
    (:then_1
      (bind _aswbp_tutorial_buddy_dialog_pannel (Utilities|Casting|CastToWBP_TutorialBuddyDialogPannel (UserInterface|GetWidget (Variables|/Game/Game/Blueprints/Tutorial/BP_TutorialBuddy.BP_TutorialBuddy_C|GetDialogBubbleWidgetComponent (Variables|Default|GetOwner)))))
      (Variables|Default|SetWidget _aswbp_tutorial_buddy_dialog_pannel))
    (:then_2
      (bind _output_get (Variables|Default|SetTypewriterComponent (Variables|/Game/Game/Blueprints/Tutorial/BP_TutorialBuddy.BP_TutorialBuddy_C|GetTypewriterText (Variables|Default|GetOwner))))
      (EventDispatchers|BindEventtoOnCompleted _output_get (delegate Custom|OnTypewriterCompleted)))))

(event Custom|StartNewDialog
  (params (Dialog%20ID :type Name))
  (CallFunction|ResetDialogValues)
  (bind _output_get (Variables|Default|SetCurrentDialogID Dialog%20ID))
  (bind _returnvalue (Utilities|GetDataTableRow (Variables|Default|GetExtraLinesDialogDataTable) _output_get)
    (:then
      (Variables|Default|SetCurrentDialogLines (.Lines (Utilities|Struct|BreakF_TuddyDialogLines _returnvalue)))
      (Variables|Default|SetCurrentDialogAudios (.Audios (Utilities|Struct|BreakF_TuddyDialogLines _returnvalue)))
      (Variables|Default|SetIsTalking? true)
      (Default|CallEDDialogStarted)
      (Default|ShowDialogBubble (Variables|Default|GetOwner))
      (CallFunction|ProcessDialog))))

(event EventBeginPlay)

(fn MoreDialogLines?
  (return (< (Variables|Default|GetCurrentDialogIndex) (- (Utilities|Array|Length (Variables|Default|GetCurrentDialogLines)) 1))))