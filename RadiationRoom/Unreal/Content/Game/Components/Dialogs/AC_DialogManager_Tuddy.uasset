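; Dialog manager component for the tutorial buddy, specialising a parent dialog manager to present its lines in the buddy's dialog bubble.
; On Init it caches the owning BP_TutorialBuddy and its bubble widget, then passes the typewriter and voice audio components to the parent before running parent initialisation.
; Its functions show or hide the bubble, send current text to the widget with typewriter effect, and load lines from a DataTable by row ID.
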(event EventInit
  (Utilities|FlowControl|Sequence
    (:then_0
      (bind _asbp_tutorial_buddy (Utilities|Casting|CastToBP_TutorialBuddy (Components|GetOwner)))
      (Variables|Default|SetOwner _asbp_tutorial_buddy))
    (:then_1
      (bind _aswbp_tutorial_buddy_dialog_pannel (Utilities|Casting|CastToWBP_TutorialBuddyDialogPannel (UserInterface|GetWidget (Variables|/Game/Game/Blueprints/Tutorial/BP_TutorialBuddy.BP_TutorialBuddy_C|GetDialogBubbleWidgetComponent (Variables|Default|GetOwner)))))
      (Variables|Default|SetWidget _aswbp_tutorial_buddy_dialog_pannel))
    (:then_2
      (CallFunction|SetTextandAudioComponents (Variables|/Game/Game/Blueprints/Tutorial/BP_TutorialBuddy.BP_TutorialBuddy_C|GetAC_TypewriterEffect (Variables|Default|GetOwner)) (Variables|/Game/Game/Blueprints/Tutorial/BP_TutorialBuddy.BP_TutorialBuddy_C|GetVoiceAudioComponent (Variables|Default|GetOwner))))
    (:then_3
      (|CallParentFunction))))

(fn ShowHideDialogWidget
  (params (ShowWidget :type Boolean))
  (bind _owner (Variables|Default|GetOwner))
  (if ShowWidget
    (Default|ShowDialogBubble _owner)
    (else
      (Default|HideDialogBubble _owner))))

(fn SetDialogText
  (params (TypewriterComponent :type AC%20Typewriter%20Effect%20Object%20Reference))
  (Default|SetDialogText (Variables|Default|GetWidget) (CallFunction|GetCurrentText) TypewriterComponent))

(fn GetDialogLinesbyID
  (params (Id :type Name :default "None"))
  (bind _returnvalue (Utilities|GetDataTableRow (Variables|Default|GetDialogDataTable) Id)
    (:then
      (Variables|Default|SetCurrentDialogs (Utilities|Struct|BreakF_DialogLineList _returnvalue)))))