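; Dialog manager component for the tutorial buddy that plays data-table dialogs as typewriter text in a speech bubble, with voice audio.
; Init caches the buddy, its bubble widget and typewriter component; StartNewDialog loads a row's lines by ID and shows the bubble.
; Each line sets text and voice from its start time; typewriter completion advances after a short delay.
; Start, stop and completion fire event dispatchers.
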(event Custom|OnTypewriterCompleted
  (if (Variables|Default|GetIsTalking?)
    (Utilities|FlowControl|Delay 1.5)
    (CallFunction|NextDialog)))

(event Custom|BindTypewriterEvents
  (EventDispatchers|BindEventtoEDonCompleted (stale Custom|Init _output_get) (delegate Custom|OnTypewriterCompleted)))

(event Custom|ProcessDialog
  (bind _owner (Variables|Default|GetOwner))
  (bind _voiceaudiocomponent (Variables|/Game/Game/Blueprints/Tutorial/BP_TutorialBuddy.BP_TutorialBuddy_C|GetVoiceAudioComponent _owner))
  (Default|SetDialogText (Variables|Default|GetWidget) (CallFunction|GetCurrentText) (Variables|Default|GetTypewriterComponent))
  (Audio|Components|Audio|SetSound _voiceaudiocomponent (CallFunction|GetCurrentVoice))
  (Audio|Components|Audio|Play _voiceaudiocomponent (CallFunction|GetCurrentTimetoStart)))

(event Custom|NextDialog
  (bind _there_are_more_dialogs (CallFunction|MoreDialogLines?))
  (if _there_are_more_dialogs
    (Variables|Default|SetCurrentDialogIndex (+ (Variables|Default|GetCurrentDialogIndex) 1))
    (CallFunction|ProcessDialog)
    (else
      (CallFunction|EndDialog))))

(event Custom|StopDialog
  (Default|HideDialogBubble (Variables|Default|GetOwner))
  (Variables|Default|SetIsTalking? false)
  (Default|CallEDDialogStopped))

(event Custom|EndDialog
  (CallFunction|ResetDialogValues)
  (Default|HideDialogBubble (Variables|Default|GetOwner))
  (Variables|Default|SetIsTalking? false)
  (Default|CallEDDialogCompleted (Variables|Default|GetCurrentDialogID))
  (Variables|Default|SetCurrentDialogID "None"))

(event Custom|ResetDialogValues
  (Utilities|Array|Clear (Variables|Default|GetCurrentDialogs))
  (Variables|Default|SetCurrentDialogIndex 0))

(event Custom|Init
  (Utilities|FlowControl|Sequence
    (:then_0
      (bind _asbp_tutorial_buddy (Utilities|Casting|CastToBP_TutorialBuddy (Components|GetOwner)))
      (Variables|Default|SetOwner _asbp_tutorial_buddy))
    (:then_1
      (bind _aswbp_tutorial_buddy_dialog_pannel (Utilities|Casting|CastToWBP_TutorialBuddyDialogPannel (UserInterface|GetWidget (Variables|/Game/Game/Blueprints/Tutorial/BP_TutorialBuddy.BP_TutorialBuddy_C|GetDialogBubbleWidgetComponent (Variables|Default|GetOwner)))))
      (Variables|Default|SetWidget _aswbp_tutorial_buddy_dialog_pannel))
    (:then_2
      (bind _output_get (Variables|Default|SetTypewriterComponent (Variables|/Game/Game/Blueprints/Tutorial/BP_TutorialBuddy.BP_TutorialBuddy_C|GetAC_TypewriterEffect (Variables|Default|GetOwner))))
      (EventDispatchers|BindEventtoEDonCompleted _output_get (delegate Custom|OnTypewriterCompleted)))))

(event Custom|StartNewDialog
  (params (Dialog%20ID :type Name))
  (CallFunction|ResetDialogValues)
  (bind _output_get (Variables|Default|SetCurrentDialogID Dialog%20ID))
  (bind _returnvalue (Utilities|GetDataTableRow (Variables|Default|GetDialogDataTable) _output_get)
    (:then
      (Variables|Default|SetCurrentDialogs (Utilities|Struct|BreakF_DialogLineList _returnvalue))
      (Variables|Default|SetIsTalking? true)
      (Default|CallEDDialogStarted)
      (Default|ShowDialogBubble (Variables|Default|GetOwner))
      (CallFunction|ProcessDialog))))

(event EventBeginPlay)

(fn MoreDialogLines?
  (return (< (Variables|Default|GetCurrentDialogIndex) (- (Utilities|Array|Length (Variables|Default|GetCurrentDialogs)) 1))))

(fn GetCurrentText
  (return (.text (Utilities|Array|Get(acopy) (Variables|Default|GetCurrentDialogs) (Variables|Default|GetCurrentDialogIndex)))))

(fn GetCurrentVoice
  (return (.voice (Utilities|Array|Get(acopy) (Variables|Default|GetCurrentDialogs) (Variables|Default|GetCurrentDialogIndex)))))

(fn GetCurrentTimetoStart
  (return (.timetostart (Utilities|Array|Get(acopy) (Variables|Default|GetCurrentDialogs) (Variables|Default|GetCurrentDialogIndex)))))