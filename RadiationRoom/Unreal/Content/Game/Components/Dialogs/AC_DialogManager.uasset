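; Dialog manager component that plays sequences of dialog lines by ID, pairing typewriter text with voice audio.
; Each line's voice starts at its own time offset, and typewriter completion advances to the next line after a short delay.
; Event dispatchers announce when dialog starts, stops or completes.
; Line lookup, text setting and widget visibility are empty functions here, and the typewriter and audio components are passed in.
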(event Custom|OnTypewriterCompleted
  (if (Variables|Default|GetIsTalking?)
    (Utilities|FlowControl|Delay 1.5)
    (CallFunction|NextDialog)))

(event Custom|BindTypewriterEvents
  (EventDispatchers|BindEventtoEDonCompleted (Variables|Default|GetTypewriterComponent) (delegate Custom|OnTypewriterCompleted)))

(event Custom|ProcessDialog
  (bind _voiceaudiocomponent (Variables|Default|GetVoiceAudioComponent))
  (CallFunction|SetDialogText (Variables|Default|GetTypewriterComponent))
  (Audio|Components|Audio|SetSound _voiceaudiocomponent (CallFunction|GetCurrentVoice))
  (Audio|Components|Audio|Play _voiceaudiocomponent (CallFunction|GetCurrentTimetoStart)))

(event Custom|NextDialog
  (if (CallFunction|MoreDialogLines?)
    (Math|Integer|IncrementInt (Variables|Default|GetCurrentDialogIndex)
      (:%20%20
        (CallFunction|ProcessDialog)))
    (else
      (CallFunction|EndDialog))))

(event Custom|StopDialog
  (CallFunction|ShowHideDialogWidget false)
  (Variables|Default|SetIsTalking? false)
  (Default|CallEDDialogStopped))

(event Custom|EndDialog
  (CallFunction|ResetDialogValues)
  (CallFunction|ShowHideDialogWidget false)
  (Variables|Default|SetIsTalking? false)
  (Default|CallEDDialogCompleted (Variables|Default|GetCurrentDialogID))
  (Variables|Default|SetCurrentDialogID "None"))

(event Custom|ResetDialogValues
  (Utilities|Array|Clear (Variables|Default|GetCurrentDialogs))
  (Variables|Default|SetCurrentDialogIndex 0))

(event Custom|Init
  (CallFunction|BindTypewriterEvents))

(event Custom|StartNewDialogByID
  (params (Dialog%20ID :type Name))
  (CallFunction|ResetDialogValues)
  (bind _output_get (Variables|Default|SetCurrentDialogID Dialog%20ID))
  (CallFunction|GetDialogLinesbyID _output_get)
  (Variables|Default|SetIsTalking? true)
  (Default|CallEDDialogStarted)
  (CallFunction|ShowHideDialogWidget true)
  (CallFunction|ProcessDialog))

(fn MoreDialogLines?
  (return (< (Variables|Default|GetCurrentDialogIndex) (- (Utilities|Array|Length (Variables|Default|GetCurrentDialogs)) 1))))

(fn GetCurrentText
  (return (.text (Utilities|Array|Get(acopy) (Variables|Default|GetCurrentDialogs) (Variables|Default|GetCurrentDialogIndex)))))

(fn GetCurrentVoice
  (return (.voice (Utilities|Array|Get(acopy) (Variables|Default|GetCurrentDialogs) (Variables|Default|GetCurrentDialogIndex)))))

(fn GetCurrentTimetoStart
  (return (.timetostart (Utilities|Array|Get(acopy) (Variables|Default|GetCurrentDialogs) (Variables|Default|GetCurrentDialogIndex)))))

(fn SetComponents
  (params (TypewriterComponent :type AC%20Typewriter%20Effect%20Object%20Reference) (VoiceAudioComponent :type Audio%20Component%20Object%20Reference))
  (Variables|Default|SetTypewriterComponent TypewriterComponent)
  (Variables|Default|SetVoiceAudioComponent VoiceAudioComponent))

(fn ShowHideDialogWidget
  (params (ShowWidget :type Boolean)))

(fn SetDialogText
  (params (TypewriterComponent :type AC%20Typewriter%20Effect%20Object%20Reference)))

(fn GetDialogLinesbyID
  (params (Id :type Name)))