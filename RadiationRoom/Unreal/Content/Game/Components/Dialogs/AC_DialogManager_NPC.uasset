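; Dialog manager component for talkable NPCs, running conversations that mix player and NPC lines.
; On init it caches the owning BP_NPC_Talkable, its dialog widget, typewriter and voice audio, then defers to the parent manager.
; The conversation index becomes a data table row name, whose lines fill parallel text and speaker-type arrays.
; Each line's type selects player or NPC text creation in the widget.
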(event Custom|NextConversation
  (if (CallFunction|MoreConversations?)
    (Math|Integer|IncrementInt (Variables|Default|GetCurrentConversationIndex))))

(event Custom|StartConversation
  (CallFunction|StartNewDialogbyID (CallFunction|ConversationIndextoID)))

(event EventInit
  (Utilities|FlowControl|Sequence
    (:then_0
      (bind _asbp_npc_talkable (Utilities|Casting|CastToBP_NPC_Talkable (Components|GetOwner)))
      (Variables|Default|SetOwner _asbp_npc_talkable))
    (:then_1
      (bind _aswbp_npcdialog (Utilities|Casting|CastToWBP_NPCDialog (UserInterface|GetWidget (Variables|/Game/Game/Blueprints/NPCs/BP_NPC_Talkable.BP_NPC_Talkable_C|GetDialogWidgetComponent (Variables|Default|GetOwner)))))
      (Variables|Default|SetWidget _aswbp_npcdialog))
    (:then_2
      (CallFunction|SetTextandAudioComponents (Variables|/Game/Game/Blueprints/NPCs/BP_NPC_Talkable.BP_NPC_Talkable_C|GetAC_TypewriterEffect (Variables|Default|GetOwner)) (Variables|/Game/Game/Blueprints/NPCs/BP_NPC.BP_NPC_C|GetVoiceAudioComponent (Variables|Default|GetOwner))))
    (:then_3
      (|CallParentFunction))))

(event EventResetDialogValues
  (|CallParentFunction)
  (Utilities|Array|Clear (Variables|Default|GetCurrentDialogType)))

(fn ShowHideDialogWidget
  (params (ShowWidget :type Boolean))
  (Default|ShowHideDialogPanel (Variables|Default|GetOwner) ShowWidget))

(fn SetDialogText
  (params (TypewriterComponent :type AC%20Typewriter%20Effect%20Object%20Reference))
  (bind _text (CallFunction|GetCurrentText))
  (bind _widget (Variables|Default|GetWidget))
  (Variables|/Game/Game/UserInterfaces/Dialogs/WBP_NPCDialog.WBP_NPCDialog_C|SetTypewriterComponent (Variables|Default|GetWidget) TypewriterComponent)
  (switch Utilities|FlowControl|Switch|SwitchonE_DialogType (CallFunction|GetCurrentDialogType)
    (:NewEnumerator0
      (Default|CreatePlayerText _widget _text))
    (:NewEnumerator1
      (Default|CreateNPCText _widget _text))))

(fn GetCurrentDialogType
  (return (Utilities|Array|Get(acopy) (Variables|Default|GetCurrentDialogType) (Variables|Default|GetCurrentDialogIndex))))

(fn MoreConversations?
  (bind _outrownames (DataTable|GetDataTableRowNames (Variables|Default|GetDialogDataTable)))
  (return (< (Variables|Default|GetCurrentDialogIndex) (- (Utilities|Array|Length _outrownames) 1))))

(fn ConversationIndextoID
  (return (Utilities|String|StringToName (Utilities|String|ToString(Integer) (Variables|Default|GetCurrentConversationIndex)))))

(fn GetDialogLinesbyID
  (params (Id :type Name :default "None"))
  (bind _returnvalue (Utilities|GetDataTableRow (Variables|Default|GetDialogDataTable) Id)
    (:then
      (for _array_element (Utilities|Struct|BreakF_DialogLines_NPC _returnvalue)
        (Utilities|Array|Add (Variables|Default|GetCurrentDialogType) (.Type (Utilities|Struct|BreakF_DialogTextAudio_NPC _array_element)))
        (Utilities|Array|Add (Variables|Default|GetCurrentDialogs) (.Line (Utilities|Struct|BreakF_DialogTextAudio_NPC _array_element)))))))