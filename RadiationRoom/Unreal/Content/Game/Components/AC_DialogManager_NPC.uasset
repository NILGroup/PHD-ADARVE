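; NPC dialog manager component that connects dialog logic to the widget and components of its owning BP_NPC_Talkable.
; On Init it caches the owner's WBP_NPCDialog from its widget component, passes the typewriter effect and voice audio components to SetComponents, then runs the parent Init.
; Panel visibility is delegated to the owner, and the current text becomes either a player or an NPC entry in the widget.
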(event EventInit
  (bind _owner (Variables|Default|GetOwner))
  (Utilities|FlowControl|Sequence
    (:then_0
      (Utilities|Casting|CastToBP_NPC_Talkable (Components|GetOwner)))
    (:then_1
      (bind _aswbp_npcdialog (Utilities|Casting|CastToWBP_NPCDialog (UserInterface|GetWidget (Variables|/Game/Game/Blueprints/Characters/BP_NPC_Talkable.BP_NPC_Talkable_C|GetDialogWidgetComponent (Variables|Default|GetOwner)))))
      (Variables|Default|SetWidget _aswbp_npcdialog))
    (:then_2
      (CallFunction|SetComponents (Variables|/Game/Game/Blueprints/Characters/BP_NPC_Talkable.BP_NPC_Talkable_C|GetAC_TypewriterEffect _owner) (Variables|/Game/Game/Blueprints/Characters/BP_NPC.BP_NPC_C|GetVoiceAudioComponent _owner)))
    (:then_3
      (|CallParentFunction))))

(fn ShowHideDialogWidget
  (params (ShowWidget :type Boolean))
  (Default|ShowHideDialogPanel (Variables|Default|GetOwner) ShowWidget))

(fn SetDialogText
  (params (TypewriterComponent :type AC%20Typewriter%20Effect%20Object%20Reference))
  (bind _text (CallFunction|GetCurrentText))
  (bind _widget (Variables|Default|GetWidget))
  (switch Utilities|FlowControl|Switch|SwitchonE_DialogType "NewEnumerator2"
    (:NewEnumerator0
      (Default|CreatePlayerText _widget _text))
    (:NewEnumerator1
      (Default|CreateNPCText _widget _text))))