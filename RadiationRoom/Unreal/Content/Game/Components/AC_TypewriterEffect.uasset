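; Typewriter effect component that reveals a given text one character at a time on a supplied text widget.
; StartTypewriting stores the settings, then UpdateText lengthens the displayed substring and re-calls itself after a delay until the full text shows, firing the OnCompleted dispatcher.
; The punctuation delay compares all but the last displayed character to the mark, so it misses most punctuation.
; DisplayedText is never reset between runs.
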(event Custom|StartTypewriting
  (params (Text :type Text) (TimePerChar :type Float%20%28double-precision%29) (TimePerPunct :type Float%20%28double-precision%29) (Text%20Widget :type Text%20Block%20Object%20Reference))
  (Utilities|FlowControl|Sequence
    (:then_0
      (Variables|Default|SetFullText (Utilities|String|ToString(Text) Text))
      (Variables|Default|SetTimePerChar TimePerChar)
      (Variables|Default|SetTimePerPunct TimePerPunct)
      (Variables|Default|SetText%20Widget Text%20Widget))
    (:then_1
      (CallFunction|UpdateText))))

(event Custom|UpdateText
  (Utilities|FlowControl|Sequence
    (:then_0
      (bind _output_get (Variables|Default|SetDisplayedText (Utilities|String|GetSubstring (Variables|Default|GetFullText) 0 (+ (Utilities|String|Len (Variables|Default|GetDisplayedText)) 1))))
      (Rendering|Components|TextRender|SetText (Variables|Default|GetText%20Widget) (Utilities|Text|ToText(String) _output_get)))
    (:then_1
      (if (Utilities|Enum|Equal(Enum) (Variables|Default|GetDisplayedText) (Variables|Default|GetFullText))
        (Default|CallEDonCompleted)
        (else
          (if (Math|Boolean|ORBoolean (Utilities|Enum|Equal(Enum) (Utilities|String|GetSubstring (Variables|Default|GetDisplayedText) 0 (- (Utilities|String|Len (Variables|Default|GetDisplayedText)) 1)) ".") (Utilities|Enum|Equal(Enum) (Utilities|String|GetSubstring (Variables|Default|GetDisplayedText) 0 (- (Utilities|String|Len (Variables|Default|GetDisplayedText)) 1)) ",") (Utilities|Enum|Equal(Enum) (Utilities|String|GetSubstring (Variables|Default|GetDisplayedText) 0 (- (Utilities|String|Len (Variables|Default|GetDisplayedText)) 1)) "?") (Utilities|Enum|Equal(Enum) (Utilities|String|GetSubstring (Variables|Default|GetDisplayedText) 0 (- (Utilities|String|Len (Variables|Default|GetDisplayedText)) 1)) "!"))
            (Utilities|FlowControl|Delay (Variables|Default|GetTimePerPunct))
            (else
              (Utilities|FlowControl|Delay (Variables|Default|GetTimePerChar))))
          (CallFunction|UpdateText))))))